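; Kamikaze enemy NPC that lights its explosive barrel while detonating and shakes the player's camera on explosion, harder when the player is hit.
; The AI controller's detonation delegate toggles emissive strength on the barrel's dynamic material.
; In the ArenaEE level, Tick cycles the mesh's vein and eye colors through a lerped rainbow palette.
; A distance-based barrel blink is present but never runs.
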(event `self.ReceiveBeginPlay`
  (bind _output (`|GetArrayItem` (`self.VeinsColors`)))
  (`parent.ReceiveBeginPlay`)
  (bind _returnvalue (`PrimitiveComponent.CreateDynamicMaterialInstance` (`self.Barrel`) 0 "/Game/Models/Skeletal/Characters/Enemies/Kamikaze/EXPLOSIVES/M_KamikazeBarrel_Inst.M_KamikazeBarrel_Inst" "None"))
  (bind _output_get (set `self.BarrelMaterial` _returnvalue))
  (bind _returnvalue_2 (`MaterialInstanceDynamic.K2_GetScalarParameterValue` _output_get "EmissiveStrength"))
  (set `self.BarrelEmissive` _returnvalue_2)
  (`MaterialInstanceDynamic.SetScalarParameterValue` _output_get "EmissiveStrength" 0.0)
  (bind _asbp_kamikaze_npc_controller (cast `/Game/Blueprints/NPCs/Kamikaze/BP_KamikazeNpcController` (`self.GetController`)))
  (add `KamikazeNpcController.OnDetonationValueChangedDelegate` _asbp_kamikaze_npc_controller (`|CreateDelegate` :!event `OnDetonationValueChanged_Event`))
  (add `NPCSubsystem.OnPlayerSpawned` (subsystem `NPCSubsystem`) (delegate `OnPlayer_Spawned_Event`))
  (add `self.OnPlayerHitByExplosionDelegate` (delegate `OnPlayerHitByExplosion_Event`))
  (bind _returnvalue_3 (`GameplayStatics.GetCurrentLevelName` true))
  (bind _output_get_2 (set `self.EnableRainbow` (`KismetStringLibrary.EqualEqual_StrStr` _returnvalue_3 "ArenaEE")))
  (if _output_get_2
    (bind _returnvalue_4 (`PrimitiveComponent.CreateDynamicMaterialInstance` (`self.Mesh`) 0 "/Game/Models/Skeletal/Characters/Enemies/Melee/material/M_MeleeEnemy_Inst.M_MeleeEnemy_Inst" "None"))
    (set `self.EnemyMat` _returnvalue_4)
    (set `self.CurrentIndex` 0)
    (set `self.NextIndex` 1)
    (set `self.LerpAlpha` 0.0)
    (`MaterialInstanceDynamic.SetVectorParameterValue` (`self.EnemyMat`) "Veins_Color" _output)
    (`MaterialInstanceDynamic.SetVectorParameterValue` (`self.EnemyMat`) "Eyes_Color" _output)))

(event `OnPlayer_Spawned_Event`
  (params (Player :type "PlayerCharacter Object Reference"))
  (set `self.PlayerTarget` Player)
  (set `self.PlayerCtrl` (`GameplayStatics.GetPlayerController` 0)))

(event `OnPlayerHitByExplosion_Event` :!signature `self.OnPlayerHitByExplosionDelegate`
  (params (bHasHitPlayer :type Boolean))
  (bind _playerctrl (`self.PlayerCtrl`))
  (if bHasHitPlayer
    (`/Game/Blueprints/Cosmetics/CameraShakeClasses/BP_CameraShaker.StrongCameraShake` _playerctrl)
    (else
      (`/Game/Blueprints/Cosmetics/CameraShakeClasses/BP_CameraShaker.WeakCameraShake` _playerctrl))))

(event `OnDetonationValueChanged_Event`
  (params (bIsDetonating :type Boolean))
  (bind _output_get (set `self.IsDetonating` bIsDetonating))
  (set `self.IsAnimating` _output_get)
  (`self.ToggleBarrelEmissive`))

(event `self.ReceiveTick`
  (params (DeltaSeconds :type "Float (single-precision)"))
  (bind _returnvalue (`KismetMathLibrary.LinearColorLerp` (`|GetArrayItem` (`self.VeinsColors`) (`self.CurrentIndex`)) (`|GetArrayItem` (`self.VeinsColors`) (`self.NextIndex`)) (`self.LerpAlpha`)))
  (if (`self.EnableRainbow`)
    (bind _output_get (set `self.LerpAlpha` (+ (`self.LerpAlpha`) (* DeltaSeconds (`self.LerpSpeed`)))))
    (if (>= _output_get 1.0)
      (set `self.LerpAlpha` 0.0)
      (set `self.CurrentIndex` (`self.NextIndex`))
      (set `self.NextIndex` (mod (+ (`self.NextIndex`) 1) (`KismetArrayLibrary.Array_Length` (`self.VeinsColors`)))))
    (`MaterialInstanceDynamic.SetVectorParameterValue` (`self.EnemyMat`) "Veins_Color" _returnvalue)
    (`MaterialInstanceDynamic.SetVectorParameterValue` (`self.EnemyMat`) "Eyes_Color" _returnvalue)))

(fn `ToggleBarrelEmissive`
  (bind _barrelmaterial (`self.BarrelMaterial`))
  (if (`self.IsAnimating`)
    (`MaterialInstanceDynamic.SetScalarParameterValue` _barrelmaterial "EmissiveStrength" (`self.BarrelEmissive`))
    (else
      (`MaterialInstanceDynamic.SetScalarParameterValue` _barrelmaterial "EmissiveStrength" 0.0))))

(fn `UserConstructionScript`)
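; Runner NPC Blueprint that gives its mesh a rainbow vein and eye effect, active only in the ArenaEE level.
; On BeginPlay it checks the level name, then creates a dynamic instance of the melee enemy material and applies the first palette color.
; Tick advances an alpha by LerpSpeed, blending both color parameters between consecutive VeinsColors entries and wrapping around the array for a continuous cycle.
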(event `self.ReceiveBeginPlay`
  (bind _output (`|GetArrayItem` (`self.VeinsColors`)))
  (bind _returnvalue (`GameplayStatics.GetCurrentLevelName` true))
  (bind _output_get (set `self.EnableRainbow` (`KismetStringLibrary.EqualEqual_StrStr` _returnvalue "ArenaEE")))
  (if _output_get
    (bind _returnvalue_2 (`PrimitiveComponent.CreateDynamicMaterialInstance` (`self.Mesh`) 0 "/Game/Models/Skeletal/Characters/Enemies/Melee/material/M_MeleeEnemy_Inst.M_MeleeEnemy_Inst" "None"))
    (set `self.EnemyMat` _returnvalue_2)
    (set `self.CurrentIndex` 0)
    (set `self.NextIndex` 1)
    (set `self.LerpAlpha` 0.0)
    (`MaterialInstanceDynamic.SetVectorParameterValue` (`self.EnemyMat`) "Veins_Color" _output)
    (`MaterialInstanceDynamic.SetVectorParameterValue` (`self.EnemyMat`) "Eyes_Color" _output)))

(event `self.ReceiveTick`
  (params (DeltaSeconds :type "Float (single-precision)"))
  (bind _returnvalue (`KismetMathLibrary.LinearColorLerp` (`|GetArrayItem` (`self.VeinsColors`) (`self.CurrentIndex`)) (`|GetArrayItem` (`self.VeinsColors`) (`self.NextIndex`)) (`self.LerpAlpha`)))
  (if (`self.EnableRainbow`)
    (bind _output_get (set `self.LerpAlpha` (+ (`self.LerpAlpha`) (* DeltaSeconds (`self.LerpSpeed`)))))
    (if (>= _output_get 1.0)
      (set `self.LerpAlpha` 0.0)
      (set `self.CurrentIndex` (`self.NextIndex`))
      (set `self.NextIndex` (mod (+ (`self.NextIndex`) 1) (`KismetArrayLibrary.Array_Length` (`self.VeinsColors`)))))
    (`MaterialInstanceDynamic.SetVectorParameterValue` (`self.EnemyMat`) "Veins_Color" _returnvalue)
    (`MaterialInstanceDynamic.SetVectorParameterValue` (`self.EnemyMat`) "Eyes_Color" _returnvalue)))

(fn `UserConstructionScript`)
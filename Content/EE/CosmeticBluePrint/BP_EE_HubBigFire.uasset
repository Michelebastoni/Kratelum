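; Cosmetic hub fire effect that switches on and off periodically once its linked arena gate opens.
; The construction script hides the Fire component, and BeginPlay unhides it in game but deactivates it and binds to the gate's opened event.
; When that event fires, Fire becomes visible and a looping timer flip-flops its activation, with Duration as the interval and Phase as the start delay offset.
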(event `self.ReceiveBeginPlay`
  (add `/Game/Blueprints/HUB_Elements/Gates/BP_ArenaGate.OnArenaGateOpened` (`self.ArenaGate`) (delegate `OnAllGatesOpened_Event`))
  (`SceneComponent.SetHiddenInGame` (`self.Fire`) false false)
  (`ActorComponent.Deactivate` (`self.Fire`)))

(event `OnAllGatesOpened_Event`
  (`SceneComponent.SetVisibility` (`self.Fire`) true false)
  (`KismetSystemLibrary.K2_SetTimerDelegate` (delegate `OnTimerDone`) (`self.Duration`) true false (`self.Phase`)))

(event `OnTimerDone`
  (bind _fire (`self.Fire`))
  (`/Engine/EditorBlueprintResources/StandardMacros.FlipFlop`
    (:`A`
      (`ActorComponent.Activate` _fire false))
    (:`B`
      (`ActorComponent.Deactivate` _fire))))

(fn `UserConstructionScript`
  (bind _fire (`self.Fire`))
  (`SceneComponent.SetHiddenInGame` _fire true false)
  (`SceneComponent.SetVisibility` _fire false false))
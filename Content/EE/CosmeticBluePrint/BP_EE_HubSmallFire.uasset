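; Cosmetic small hub fire that stays inactive until its linked ArenaGate reports all collectibles destroyed.
; The fire then activates and a timeline scales it up non-uniformly, with a Z multiplier randomized at BeginPlay.
; Afterwards, a looping timer with a varied start delay drives a FlipFlop that toggles the fire on and off.
; The construction script hides the Fire component until BeginPlay.
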(event `self.ReceiveBeginPlay`
  (bind _fire (`self.Fire`))
  (add `/Game/Blueprints/HUB_Elements/Gates/BP_ArenaGate.OnAllCollectiblesDestroyed` (`self.ArenaGate`) (delegate `OnArenaGateOpened_Event`))
  (`SceneComponent.SetHiddenInGame` _fire false false)
  (`SceneComponent.SetVisibility` _fire true false)
  (`ActorComponent.Deactivate` (`self.Fire`))
  (set `self.RandomizedZScale` (`KismetMathLibrary.RandomFloatInRange` 1.5 2.5)))

(event `OnArenaGateOpened_Event`
  (`ActorComponent.Activate` (`self.Fire`) true)
  (bind (_direction _scalelerp) (`Timeline|LerpScaleTimeline`)
    (:`Update`
      (`SceneComponent.SetRelativeScale3D` (`self.Fire`) (`KismetMathLibrary.MakeVector` (* _scalelerp 0.25) _scalelerp (* _scalelerp (`self.RandomizedZScale`)))))
    (:`Finished`
      (`KismetSystemLibrary.K2_SetTimerDelegate` (delegate `OnTimerDone`) (`self.Duration`) true false 1.0 0.75))))

(event `OnTimerDone`
  (bind _fire (`self.Fire`))
  (`/Engine/EditorBlueprintResources/StandardMacros.FlipFlop`
    (:`A`
      (`ActorComponent.Activate` _fire false))
    (:`B`
      (`ActorComponent.Deactivate` _fire))))

(fn `UserConstructionScript`
  (bind _fire (`self.Fire`))
  (`SceneComponent.SetHiddenInGame` _fire true false)
  (`SceneComponent.SetVisibility` _fire false false))
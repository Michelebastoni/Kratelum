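; Dispatcher in the EE arena set that unlocks trap buttons one at a time as levels are won.
; On BeginPlay it loads the first KillToUnlock threshold into EnemiesToKill and binds to the level-won delegate.
; Each win unlocks the current button if valid and still locked, then advances the index, clamped to the last threshold, and updates EnemiesToKill.
; Kill counting is not handled in this graph.
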(event `self.ReceiveBeginPlay`
  (set `self.EnemiesToKill` (`|GetArrayItem` (`self.KillToUnlock`)))
  (add `self.OnLevelWonDelegate` (delegate `OnLevelWonDelegate_Event`)))

(event `OnLevelWonDelegate_Event` :!signature `self.OnLevelWonDelegate`
  (params (LevelIndex :type Integer))
  (bind _killtounlock (`self.KillToUnlock`))
  (bind _output (`|GetArrayItem` (`self.BP_EETrapButton`) (`self.KillToUnlockIndex`)))
  (`/Engine/EditorBlueprintResources/StandardMacros.IsValid` _output
    (:`Is Valid`
      (if (not (`/Game/EE/Traps/BP_EE_TrapButton.IsUnlock` _output))
        (set `/Game/EE/Traps/BP_EE_TrapButton.IsUnlock` true _output)
        (bind _result (`/Engine/EditorBlueprintResources/StandardMacros.IncrementInt` (`self.KillToUnlockIndex`))
          (:`  `
            (bind _output_get (set `self.KillToUnlockIndex` (`KismetMathLibrary.Min` (- (`KismetArrayLibrary.Array_Length` _killtounlock) 1) _result)))
            (set `self.EnemiesToKill` (`|GetArrayItem` _killtounlock _output_get))))))))

(fn `UserConstructionScript`)
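; Arena dispatcher that lights ritual fires one after another as successive kill thresholds are met.
; It seeds EnemiesToKill from the first KillToUnlock entry and listens to the level-won delegate.
; Each win activates the inactive fire at the current index, then advances the index, clamped to the last threshold, and loads that value as the next kill target.
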(event `self.ReceiveBeginPlay`
  (set `self.EnemiesToKill` (`|GetArrayItem` (`self.KillToUnlock`)))
  (add `self.OnLevelWonDelegate` (delegate `OnLevelWonDelegate_Event`)))

(event `OnLevelWonDelegate_Event` :!signature `self.OnLevelWonDelegate`
  (params (LevelIndex :type Integer))
  (bind _killtounlock (`self.KillToUnlock`))
  (bind _output (`|GetArrayItem` (`self.BP_EERitualFire`) (`self.KillToUnlockIndex`)))
  (`/Engine/EditorBlueprintResources/StandardMacros.IsValid` _output
    (:`Is Valid`
      (if (not (`/Game/EE/CosmeticBluePrint/BP_RitualFire.IsActivate` _output))
        (set `/Game/EE/CosmeticBluePrint/BP_RitualFire.IsActivate` true _output)
        (`/Game/EE/CosmeticBluePrint/BP_RitualFire.ActivateRitualFire` _output)
        (`/Engine/EditorBlueprintResources/StandardMacros.IncrementInt` (`self.KillToUnlockIndex`)
          (:`  `
            (bind _output_get (set `self.KillToUnlockIndex` (`KismetMathLibrary.Min` (- (`KismetArrayLibrary.Array_Length` _killtounlock) 1) (`self.KillToUnlockIndex`))))
            (set `self.EnemiesToKill` (`|GetArrayItem` _killtounlock _output_get))))))))

(fn `UserConstructionScript`)
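; BP_EE_Eye is an Easter-egg collectible eye that stays hidden until its linked ArenaGate reports all gates opened.
; Once revealed, its interaction trigger activates, and a player interaction notifies the gate, plays a sound, spawns a fire Niagara effect and destroys the actor.
; A randomly delayed timeline bobs the eye vertically by adding scaled world offsets on each update.
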(event `self.ReceiveBeginPlay`
  (`parent.ReceiveBeginPlay`)
  (set `PrimitiveComponent.bGenerateOverlapEvents` false (`self.InteractionTrigger`))
  (`self.SetActorHiddenInGame` true)
  (add `/Game/Blueprints/HUB_Elements/Gates/BP_ArenaGate.OnAllGatesOpened` (`self.ArenaGate`) (delegate `OnAllGatesOpened_Event`))
  (`KismetSystemLibrary.Delay` (`KismetMathLibrary.RandomFloatInRange` 0.0 1.5))
  (bind (_direction _move) (`Timeline|MoveUpDown`)
    (:`Update`
      (`SceneComponent.K2_AddWorldOffset` (`self.Eye`) (`KismetMathLibrary.MakeVector` 0.0 0.0 (* _move (`self.VerticalOffsetMultiplier`))) false false))))

(event `OnAllGatesOpened_Event`
  (`self.SetActorHiddenInGame` false)
  (set `PrimitiveComponent.bGenerateOverlapEvents` true (`self.InteractionTrigger`)))

(event `self.Interact`
  (params (Interactor :type "Interactor Interface (by ref)") (InteractionMethod :type "EInteractionMethod Enum" :default "KeyPress"))
  (bind _asinteraction_component (cast `InteractionComponent` (`KismetSystemLibrary.Conv_InterfaceToObject` Interactor)))
  (cast `PlayerCharacter` (`ActorComponent.GetOwner` _asinteraction_component))
  (bind _arenagate (`self.ArenaGate`)
    (:`then`
      (`/Game/Blueprints/HUB_Elements/Gates/BP_ArenaGate.On Arena EECollectible Destroyed` _arenagate)
      (`GameplayStatics.PlaySound2D` "/Game/Audio/SFX/UI/SFX_UI_Button_Press.SFX_UI_Button_Press" 1.0 1.0 0.0 null null)
      (`NiagaraFunctionLibrary.SpawnSystemAtLocation` "/Game/EE/VFX/NS_EE_Eye_Fire.NS_EE_Eye_Fire" (`self.K2_GetActorLocation`))
      (`KismetSystemLibrary.DelayUntilNextTick`)
      (`self.K2_DestroyActor`))
    (:`else`)))

(fn `UserConstructionScript`)
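; BP_EE_TargetPoint is a trap target marker that shows a ring decal tracking the countdown to the next loop trap spawn.
; On BeginPlay it hides the inactive-trap decal if active, caches the spline transform and applies a dynamic ring material to its decal.
; A near-per-frame looping timer sets Ring_Percentage to the EELoopTraps spawn timer's remaining time divided by SpawnTime while that timer handle is valid.
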(event `self.ReceiveBeginPlay`
  (if (`self.IsActive`)
    (`SceneComponent.SetHiddenInGame` (`self.DecalInactiveTrap`) true false))
  (set `self.SplineTransform` (`SceneComponent.K2_GetComponentToWorld` (`/Game/EE/Traps/BP_SplineActor.Spline` (`self.SplinePath`))))
  (bind _returnvalue (`KismetMaterialLibrary.CreateDynamicMaterialInstance` "/Game/Materials/Magazine_Ring/MI_EETargetRing.MI_EETargetRing"))
  (bind _output_get (set `self.MagazineRing` _returnvalue))
  (`DecalComponent.SetDecalMaterial` (`self.Decal`) _output_get)
  (`KismetSystemLibrary.K2_SetTimerDelegate` (delegate `UpdateRing`) 0.0001 true))

(event `UpdateRing`
  (bind _eelooptraps (`self.EELoopTraps`))
  (bind _looptrapspawnhandle (`/Game/EE/Traps/BP_EE_LoopTraps.LoopTrapSpawnHandle` _eelooptraps))
  (if (`KismetSystemLibrary.K2_IsValidTimerHandle` _looptrapspawnhandle)
    (`self.SetRingValue` (/ (`KismetSystemLibrary.K2_GetTimerRemainingTimeHandle` _looptrapspawnhandle) (`/Game/EE/Traps/BP_EE_LoopTraps.SpawnTime` _eelooptraps)))))

(fn `SetRingValue`
  (params (Value :type "Float (single-precision)"))
  (`MaterialInstanceDynamic.SetScalarParameterValue` (`self.MagazineRing`) "Ring_Percentage" Value))

(fn `UserConstructionScript`)
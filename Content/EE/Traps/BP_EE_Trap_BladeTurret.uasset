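; Blade turret trap that relies on its parent class for its behavior and takes a spline as its path.
; SetPath stores the spline in Path, and BeginPlay and Tick call their parent versions only while Path is valid.
; A Path assigned after BeginPlay lets parent Tick run, but the skipped parent BeginPlay is not replayed.
; The construction script only calls the parent's.
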(event `self.ReceiveBeginPlay`
  (`/Engine/EditorBlueprintResources/StandardMacros.IsValid` (`self.Path`)
    (:`Is Valid`
      (`parent.ReceiveBeginPlay`))))

(event `self.ReceiveTick`
  (params (DeltaSeconds :type "Float (single-precision)"))
  (`/Engine/EditorBlueprintResources/StandardMacros.IsValid` (`self.Path`)
    (:`Is Valid`
      (`parent.ReceiveTick` DeltaSeconds))))

(event `/Game/Blueprints/Arena_Prototyping/Traps/Interfaces/BPI_PathFollowingTrap.SetPath`
  (params (Spline :type "SplineComponent Object Reference"))
  (set `self.Path` Spline))

(fn `UserConstructionScript`
  (`parent.UserConstructionScript`))
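; BP_EE_Trap_InfiniteDash is a trap actor that grants the SteveJr character a timed infinite dash when touched.
; ToggleTrap switches it on and activates its decal effect; despite the name, it never switches it off.
; While active, each box overlap by SteveJr plays a sound, enables the dash for the configured duration and shows the power-up sign on the HUD.
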(event `self.BoxCollision.OnComponentBeginOverlap`
  (params (OverlappedComponent :type "PrimitiveComponent Object Reference") (OtherActor :type "Actor Object Reference") (OtherComp :type "PrimitiveComponent Object Reference") (OtherBodyIndex :type Integer) (bFromSweep :type Boolean) (SweepResult :type "HitResult Structure (by ref)"))
  (if (`self.bIsActive`)
    (bind _assteve_jr (cast `/Game/Blueprints/Character_Test/SteveJr` OtherActor))
    (`GameplayStatics.PlaySound2D` (`self.Sound`) 1.0 1.0 0.0 null null)
    (`PlayerCharacter.EnableInfiniteDash` _assteve_jr (`self.InfiniteDashDuration`))
    (`/Game/Blueprints/Widgets/PowerUPSign_Widget/WBP_PowerUpSign.ShowCollectible` (`/Game/Blueprints/Widgets/BPW_HUD.WBP_PowerUpSign` (`/Game/Blueprints/Character_Test/SteveJr.HUD` _assteve_jr)) "NewEnumerator0" (`self.InfiniteDash`))))

(event `self.ToggleTrap`
  (set `self.bIsActive` true)
  (`ActorComponent.Activate` (`self.NS_InfiniteDashDecal`) false))

(fn `UserConstructionScript`)
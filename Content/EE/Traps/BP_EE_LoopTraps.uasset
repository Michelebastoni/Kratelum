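; BP_EE_LoopTraps periodically activates a set of linked trap buttons on a repeating timer.
; After a starting delay, each cycle plays a warning sound, then reveals every unlocked button's mesh, clears its traps and turns its decal target active.
; StopSpawningTraps disables further activation, destroys all traps on the linked buttons and clears the looping timer.
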(event `self.ReceiveBeginPlay`
  (`KismetSystemLibrary.Delay` (`self.StartingSpawnDelay`))
  (`self.ActivateTraps`)
  (bind _returnvalue (`KismetSystemLibrary.K2_SetTimerDelegate` (delegate `ActivateTraps`) (`self.SpawnTime`) true))
  (set `self.LoopTrapSpawnHandle` _returnvalue))

(event `ActivateTraps`
  (if (`self.CanSpawn`)
    (`GameplayStatics.PlaySound2D` (`self.WarningSound`) 1.0 1.0 0.0 null null)
    (for _array_element (`self.LinkedTrapButtons`)
      (`/Engine/EditorBlueprintResources/StandardMacros.IsValid` _array_element
        (:`Is Valid`
          (if (`/Game/EE/Traps/BP_EE_TrapButton.IsUnlock` _array_element)
            (`SceneComponent.SetHiddenInGame` (`/Game/EE/Traps/BP_EE_TrapButton.SkeletalMesh` _array_element) false false)
            (`/Game/EE/Traps/BP_EE_TrapButton.ClearTraps` _array_element)
            (`/Game/EE/Traps/BP_EE_TrapButton.TurnDecalTargetActive` _array_element)))))))

(event `StopSpawningTraps`
  (set `self.CanSpawn` false)
  (for _array_element (`self.LinkedTrapButtons`)
    (`/Game/EE/Traps/BP_EE_TrapButton.DestroyAllTraps` _array_element)
    (`KismetSystemLibrary.K2_ClearAndInvalidateTimerHandle` (`self.LoopTrapSpawnHandle`))))

(fn `UserConstructionScript`)
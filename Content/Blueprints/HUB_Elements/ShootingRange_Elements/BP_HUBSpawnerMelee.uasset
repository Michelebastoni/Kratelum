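; Shooting range spawner in the HUB that places melee enemies at designated spawn point actors.
; On BeginPlay it sets an interaction cooldown, takes the spawn points from the keys of SpawnEnemyMap and fires the spawn event.
; The event spawns EnemyToSpawn only at points without a valid enemy, recording each new NpcBase in the map.
; ToggleTraps extends the parent behavior by firing the spawn event again to refill empty points.
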(event `self.ReceiveBeginPlay`
  (`parent.ReceiveBeginPlay`)
  (set `self.InteractionCooldown` 1.0)
  (bind _keys (`BlueprintMapLibrary.Map_Keys` (`self.SpawnEnemyMap`)))
  (set `self.SpawnLocations` _keys)
  (`self.SpawnEnemy_Event` null))

(event `SpawnEnemy_Event`
  (params (SpawnPos :type "BillboardComponent Object Reference"))
  (bind _spawnenemymap (`self.SpawnEnemyMap`))
  ;[1 0.7104 0.5684] Spawn Event
  (for _array_element (`self.SpawnLocations`)
    (`/Engine/EditorBlueprintResources/StandardMacros.IsValid` (`BlueprintMapLibrary.Map_Find` _spawnenemymap _array_element)
      (:`Is Not Valid`
        (bind _returnvalue (`|SpawnActorFromClass` (`self.Enemy To Spawn`) (`KismetMathLibrary.MakeTransform` (`self.K2_GetActorLocation` _array_element)) "AlwaysSpawn" "MultiplyWithRoot" null null))
        (`/Engine/EditorBlueprintResources/StandardMacros.IsValid` _returnvalue
          (:`Is Valid`
            (bind _asnpc_base (cast `NpcBase` _returnvalue))
            (`BlueprintMapLibrary.Map_Add` _spawnenemymap _array_element _asnpc_base)))))))

(fn `ToggleTraps`
  (`parent.ToggleTraps`)
  (`self.SpawnEnemy_Event` null)
  (`self.SpawnEnemy_Event` null))

(fn `UserConstructionScript`
  (`parent.UserConstructionScript`))
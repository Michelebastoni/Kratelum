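; HUB shooting range button that, when shot, swaps the trap linked to a TrapButton for the next in TrapsArray.
; It destroys the linked traps, including any barrel spawner's current barrel, then spawns the next at its index-matched spawn point and links it.
; A timeline, emissive material, Niagara effect and sounds give press feedback, and a delay after spawning resets both buttons.
; BeginPlay spawns the first trap.
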(event `self.ReceiveBeginPlay`
  (set `self.BtnStartingLocation` (`SceneComponent.RelativeLocation` (`self.Button`)))
  (set `self.TrapIndex` 1)
  (set `self.IsBeginPlay` true)
  (`self.SpawnCurrentTrap`))

(event `self.Interact`
  (params (Interactor :type "Interactor Interface (by ref)") (InteractionMethod :type "EInteractionMethod Enum" :default "KeyPress"))
  (bind _trapindex (`self.TrapIndex`))
  (set `self.IsBeginPlay` false)
  (if (not (`self.IsActive`))
    (`GameplayStatics.PlaySoundAtLocation` (`self.ActivationSound`) (0.0 0.0 0.0) (struct) 1.0 1.0 0.0 null null null null)
    (`self.TurnOnButton`)
    (set `self.IsActive` true)
    (`/Engine/EditorBlueprintResources/StandardMacros.IncrementInt` _trapindex
      (:`  `
        (if (> _trapindex (`KismetArrayLibrary.Array_Length` (`self.TrapsArray`)))
          (set `self.TrapIndex` 1))
        (switch `EInteractionMethod` InteractionMethod
          (:`Shooting`
            (bind _trapbutton (`self.TrapButton`)
              (:`then`
                (bind _linkedtraps (`/Game/Blueprints/Arena_Prototyping/Traps/BP_TrapButton.LinkedTraps` _trapbutton))
                (for _array_element _linkedtraps
                  (`/Engine/EditorBlueprintResources/StandardMacros.IsValid` _array_element
                    (:`Is Valid`
                      (if (== (`GameplayStatics.GetObjectClass` _array_element) "/Game/Blueprints/Arena_Prototyping/Traps/HUB_Traps/BP_HUB_Trap_BarrelSpawner.BP_HUB_Trap_BarrelSpawner_C")
                        (bind _asbp_trap_barrel_spawner (cast `/Game/Blueprints/Arena_Prototyping/Traps/BP_Trap_BarrelSpawner` _array_element))
                        (bind _currentbarrel (`/Game/Blueprints/Arena_Prototyping/Traps/BP_Trap_BarrelSpawner.CurrentBarrel` _asbp_trap_barrel_spawner))
                        (`/Engine/EditorBlueprintResources/StandardMacros.IsValid` _currentbarrel
                          (:`Is Valid`
                            (`self.K2_DestroyActor` _currentbarrel))
                          (:`Is Not Valid`
                            _)))
                      (`self.K2_DestroyActor` _array_element))))
                (`KismetArrayLibrary.Array_Clear` _linkedtraps)
                (`self.SpawnCurrentTrap`))
              (:`else`))))))))

(event `SpawnCurrentTrap`
  (bind _trapbutton (`self.TrapButton`))
  (bind _returnvalue (- (`self.TrapIndex`) 1))
  (bind _returnvalue_2 (`|SpawnActorFromClass` (`|GetArrayItem` (`self.TrapsArray`) _returnvalue) (`KismetMathLibrary.MakeTransform` (select `int` _returnvalue :`0` (`SceneComponent.K2_GetComponentLocation` (`self.SpawnPoint_1`)) :`1` (`SceneComponent.K2_GetComponentLocation` (`self.SpawnPoint_2`)) :`2` (`SceneComponent.K2_GetComponentLocation` (`self.SpawnPoint_3`)) :`3` (`SceneComponent.K2_GetComponentLocation` (`self.SpawnPoint_4`)))) "AlwaysSpawn" "MultiplyWithRoot" null null))
  (bind _trapbutton_2 (`self.TrapButton`)
    (:`then`
      (`KismetArrayLibrary.Array_Add` (`/Game/Blueprints/Arena_Prototyping/Traps/BP_TrapButton.LinkedTraps` _trapbutton_2) _returnvalue_2)
      (`KismetSystemLibrary.Delay` 2.5)
      (`self.TurnOffButton`)
      (set `/Game/Blueprints/Arena_Prototyping/Traps/BP_TrapButton.bIsActive` false _trapbutton)
      (`/Game/Blueprints/Arena_Prototyping/Traps/BP_TrapButton.TurnOffButton` _trapbutton))
    (:`else`)))

(event `TurnOnButton`
  (bind (_btnstartinglocation_x _btnstartinglocation_y _btnstartinglocation_z) (`KismetMathLibrary.BreakVector` (`self.BtnStartingLocation`)))
  (`ActorComponent.Activate` (`self.Niagara`) true)
  (`MaterialInstanceDynamic.SetScalarParameterValue` (`self.Button Material`) (`self.Name Emissive`) 0.0)
  (bind (_direction _alpha) (`Timeline|Timeline` :!via `PlayFromStart` :!label _label)
    (:`Update`
      (`SceneComponent.K2_SetRelativeLocation` (`self.Button`) (`KismetMathLibrary.MakeVector` (+ (`KismetMathLibrary.Lerp` 0.0 -10.0 _alpha) _btnstartinglocation_x) _btnstartinglocation_y _btnstartinglocation_z) false false))
    (:`Finished`
      (switch `ETimelineDirection` _direction
        (:`Backward`
          (set `self.IsActive` false))))))

(event `TurnOffButton`
  (if (not (`self.IsBeginPlay`))
    (`GameplayStatics.PlaySoundAtLocation` (`self.DeactivationSound`) (0.0 0.0 0.0) (struct) 1.0 1.0 0.0 null null null null))
  (`MaterialInstanceDynamic.SetScalarParameterValue` (`self.Button Material`) (`self.Name Emissive`) (`self.BtnEmissiveIntensity`))
  (`ActorComponent.Activate` (`self.Niagara`) false)
  (goto _label :!via `ReverseFromEnd`))

(fn `UserConstructionScript`
  (bind _returnvalue (`PrimitiveComponent.CreateDynamicMaterialInstance` (`self.Button`) 0 "/Game/Materials/SolidColors/M_SolidEmissive_Red.M_SolidEmissive_Red" "None"))
  (set `self.Button Material` _returnvalue)
  (`MaterialInstanceDynamic.SetScalarParameterValue` _returnvalue (`self.Name Emissive`) (`self.BtnEmissiveIntensity`)))
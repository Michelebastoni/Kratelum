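; BP_HUBMelee is a poolable melee character for the HUB shooting range.
; Pool events set the pool-actor flag, change the in-use state, or return the character to the pool.
; SetInUseFunc toggles collision, movement avoidance, visibility and ticking together, and shows or hides any valid current weapon to match.
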(event `self.SetIsInUse`
  (params (bIsInUse :type Boolean))
  ;[0.3216 0.6196 0.6824] Pool
  (`self.SetInUse_Func` bIsInUse))

(event `self.ReturnToPool`
  ;[0.3216 0.6196 0.6824] Pool
  (`self.SetInUse_Func` false))

(event `self.SetIsPoolActor`
  (params (bIsPoolActor :type Boolean))
  ;[0.3216 0.6196 0.6824] Pool
  (set `self.bIsPoolActor` bIsPoolActor))

(fn `SetInUse_Func`
  (params (bIsInUse :type Boolean))
  (bind _returnvalue (`self.GetCurrentWeapon`))
  (set `self.bIsInUse` bIsInUse)
  (`self.SetActorEnableCollision` (`local.bIsInUse`))
  (`CharacterMovementComponent.SetAvoidanceEnabled` (`self.CharacterMovement`) (`local.bIsInUse`))
  (`self.SetActorHiddenInGame` (not (`local.bIsInUse`)))
  (`/Engine/EditorBlueprintResources/StandardMacros.IsValid` _returnvalue
    (:`Is Valid`
      (`self.SetActorHiddenInGame` _returnvalue (not (`local.bIsInUse`))))
    (:`Is Not Valid`
      _))
  (`self.SetActorTickEnabled` (`local.bIsInUse`)))

(fn `UserConstructionScript`)
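; BP_HUBWeaponSpawner spawns weapons at target points for the HUB shooting range.
; On ToggleTraps, if no valid CurrentActor exists, it loops over TargetPoints, spawning WeaponVariants classes there and advancing a wrapping index after each spawn.
; CurrentActor keeps only the last spawned actor, blocking further spawns while it remains valid.
; CanInteract always returns false, so direct interaction is disabled, and BeginPlay zeroes the inherited interaction cooldown.
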(event `self.ReceiveBeginPlay`
  (`parent.ReceiveBeginPlay`)
  (set `self.InteractionCooldown` 0.0))

(event `self.ToggleTraps`
  (bind _output (`|GetArrayItem` (`self.WeaponVariants`) (`self.WeaponIndex`)))
  (`/Engine/EditorBlueprintResources/StandardMacros.IsValid` (`self.CurrentActor`)
    (:`Is Not Valid`
      (for _array_element (`self.TargetPoints`)
        (if (`KismetSystemLibrary.IsValidClass` _output)
          (bind _returnvalue (`|SpawnActorFromClass` _output (`KismetMathLibrary.MakeTransform` (`SceneComponent.K2_GetComponentLocation` (`Actor.RootComponent` _array_element))) "AlwaysSpawn" "MultiplyWithRoot" null null))
          (set `self.CurrentActor` _returnvalue)
          (`/Engine/EditorBlueprintResources/StandardMacros.IncrementInt` (`self.WeaponIndex`)
            (:`  `
              (if (>= (`self.WeaponIndex`) (`KismetArrayLibrary.Array_Length` (`self.WeaponVariants`)))
                (set `self.WeaponIndex` 0)))))))))

(fn `CanInteract`
  (params (Interactor :type "Interactor Interface (by ref)") (InteractionMethod :type "EInteractionMethod Enum" :default "KeyPress"))
  (returns (ReturnValue :type Boolean))
  (return false))

(fn `UserConstructionScript`)
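; Hub arena gate that stays hidden until all its linked buttons are activated and enough collectibles are destroyed, then loads its level on overlap.
; Button and collectible counters feed PerformChecks, which enables the trigger, hides a linked light and broadcasts the opening.
; Opening reveals the gate meshes and score widget after a lightning flash, then loops randomized directional-light flicker with thunder audio.
; BeginPlay also adds an eye-counter widget bound to the gate.
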(event `self.ReceiveBeginPlay`
  (for _array_element (`self.GateButtons`)
    (add `/Game/Blueprints/HUB_Elements/Gates/BP_OpenLevelButton.OnLevelButtonActivated` _array_element (delegate `OnLevelButtonActivated_Event`)))
  (`PrimitiveComponent.SetCollisionEnabled` (`self.TriggerBox`) "NoCollision")
  (`SceneComponent.SetHiddenInGame` (`self.SM_BiggerGate`) true false)
  (`SceneComponent.SetHiddenInGame` (`self.SM_SmallerGate`) true false)
  (`SceneComponent.SetHiddenInGame` (`/Game/Blueprints/RnD/BP_ScoreViewer.Widget` (`self.ScoreViewer`)) true false)
  (add `self.OnArenaGateOpened` (delegate `OnArenaGateOpened_Event`))
  (bind _returnvalue (`|CreateWidget` "/Game/EE/UI/BPW_EyeCounter.BPW_EyeCounter_C" (`GameplayStatics.GetPlayerController` 0)))
  (`UserWidget.AddToViewport` _returnvalue 0)
  (`/Game/EE/UI/BPW_EyeCounter.Setup` _returnvalue self))

(event `OnLevelButtonActivated_Event`
  (bind _result (`/Engine/EditorBlueprintResources/StandardMacros.IncrementInt` (`self.CurrentOpenGates`))
    (:`  `
      (if (== _result (`KismetArrayLibrary.Array_Length` (`self.GateButtons`)))
        (`self.OnAllGatesOpened`)
        (`self.PerformChecks`)))))

(event `OnArenaGateOpened_Event`
  (bind _returnvalue (`KismetMathLibrary.RandomFloatInRange` 0.1 0.3))
  (bind _directionallight (`self.DirectionalLight`))
  (bind _directionallight_2 (`self.DirectionalLight`))
  (`SceneComponent.SetVisibility` (`self.DirectionalLight`) true false)
  (`SceneComponent.SetHiddenInGame` _directionallight_2 false false)
  (`KismetSystemLibrary.Delay` _returnvalue)
  (`SceneComponent.SetHiddenInGame` _directionallight_2 true false)
  (`KismetSystemLibrary.Delay` _returnvalue)
  (`SceneComponent.SetHiddenInGame` _directionallight_2 false false)
  (`KismetSystemLibrary.Delay` _returnvalue)
  (`SceneComponent.SetHiddenInGame` _directionallight_2 true false)
  (`KismetSystemLibrary.Delay` _returnvalue)
  (`SceneComponent.SetHiddenInGame` _directionallight false false)
  (`KismetSystemLibrary.Delay` _returnvalue)
  (`SceneComponent.SetHiddenInGame` _directionallight true false)
  (`KismetSystemLibrary.Delay` _returnvalue)
  (`SceneComponent.SetHiddenInGame` _directionallight false false)
  (`KismetSystemLibrary.Delay` _returnvalue)
  (`SceneComponent.SetHiddenInGame` _directionallight true false)
  (`KismetSystemLibrary.Delay` _returnvalue)
  (`GameplayStatics.PlaySound2D` "/Game/Audio/SFX/0_Game/GameplayFeedbacks/ThunderStruck_Cue.ThunderStruck_Cue" 1.0 1.0 0.0 null null)
  (`KismetSystemLibrary.Delay` 1.5)
  (`SceneComponent.SetHiddenInGame` (`self.SM_BiggerGate`) false false)
  (`SceneComponent.SetHiddenInGame` (`self.SM_SmallerGate`) false false)
  (`SceneComponent.SetHiddenInGame` (`/Game/Blueprints/RnD/BP_ScoreViewer.Widget` (`self.ScoreViewer`)) false false)
  (`KismetSystemLibrary.K2_SetTimerDelegate` (delegate `PersistentThunders`) 2.0 true))

(event `self.TriggerBox.OnComponentBeginOverlap`
  (params (OverlappedComponent :type "PrimitiveComponent Object Reference") (OtherActor :type "Actor Object Reference") (OtherComp :type "PrimitiveComponent Object Reference") (OtherBodyIndex :type Integer) (bFromSweep :type Boolean) (SweepResult :type "HitResult Structure (by ref)"))
  (`GameplayStatics.OpenLevelBySoftObjectPtr` (`self.Level`)))

(event `PersistentThunders`
  (bind _returnvalue (`KismetMathLibrary.RandomFloatInRange` 0.1 0.6))
  (bind _directionallight (`self.DirectionalLight`))
  (bind _directionallight_2 (`self.DirectionalLight`))
  (`SceneComponent.SetHiddenInGame` _directionallight_2 false false)
  (`KismetSystemLibrary.Delay` _returnvalue)
  (`SceneComponent.SetHiddenInGame` _directionallight_2 true false)
  (`KismetSystemLibrary.Delay` _returnvalue)
  (`SceneComponent.SetHiddenInGame` _directionallight_2 false false)
  (`KismetSystemLibrary.Delay` _returnvalue)
  (`SceneComponent.SetHiddenInGame` _directionallight_2 true false)
  (`KismetSystemLibrary.Delay` _returnvalue)
  (`SceneComponent.SetHiddenInGame` _directionallight false false)
  (`KismetSystemLibrary.Delay` _returnvalue)
  (`SceneComponent.SetHiddenInGame` _directionallight true false)
  (`KismetSystemLibrary.Delay` _returnvalue)
  (`SceneComponent.SetHiddenInGame` _directionallight false false)
  (`KismetSystemLibrary.Delay` _returnvalue)
  (`SceneComponent.SetHiddenInGame` _directionallight true false)
  (`KismetSystemLibrary.Delay` _returnvalue)
  (`GameplayStatics.PlaySound2D` "/Game/Audio/SFX/0_Game/GameplayFeedbacks/ThunderStruck_Cue.ThunderStruck_Cue" 1.5 1.0 0.0 null null)
  (`KismetSystemLibrary.Delay` (`KismetMathLibrary.RandomFloatInRange` 1.0 2.0)))

(fn `On Arena EECollectible Destroyed`
  (bind _result (`/Engine/EditorBlueprintResources/StandardMacros.IncrementInt` (`self.DestroyedObjects`))
    (:`  `
      (`self.OnCollectibleDestroyed`)
      (if (== _result (`self.ObjectsToDestroy`))
        (`self.OnAllCollectiblesDestroyed`)
        (`self.PerformChecks`)))))

(fn `PerformChecks`
  (if (and (== (`self.CurrentOpenGates`) (`KismetArrayLibrary.Array_Length` (`self.GateButtons`))) (== (`self.ObjectsToDestroy`) (`self.DestroyedObjects`)))
    (`PrimitiveComponent.SetCollisionEnabled` (`self.TriggerBox`) "QueryOnly")
    (`SceneComponent.SetHiddenInGame` (`Light.LightComponent` (`self.LightToTurnOff`)) true false)
    (`self.OnArenaGateOpened`)))

(fn `UserConstructionScript`)
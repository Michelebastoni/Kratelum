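; Hub quit button that opens a temporary portal, which closes the game when entered.
; Interact presses the button with a Timeline, zeroes its dynamic material emissive, plays Niagara effects and reveals the portal meshes.
; After TimeToDisappear it reverses the press, restores the glow and hides the portal.
; A box overlap during that active window calls QuitGame after a short delay; CanInteract always returns false.
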(event `self.ReceiveBeginPlay`
  (set `self.BtnStartingLocation` (`SceneComponent.RelativeLocation` (`self.Button`)))
  (bind _returnvalue (`PrimitiveComponent.CreateDynamicMaterialInstance` (`self.Button`) 0 "/Game/Materials/SolidColors/M_SolidEmissive_Red.M_SolidEmissive_Red" "None"))
  (bind _output_get (set `self.ButtonEmissiveMat` _returnvalue))
  (bind _returnvalue_2 (`MaterialInstanceDynamic.K2_GetScalarParameterValue` _output_get (`self.NameEmissive`)))
  (set `self.BtnEmissiveIntensity` _returnvalue_2))

(event `self.Interact`
  (params (Interactor :type "Interactor Interface (by ref)") (InteractionMethod :type "EInteractionMethod Enum" :default "KeyPress"))
  (if (not (`self.isActive`))
    (set `self.isActive` true)
    (`ActorComponent.Activate` (`self.NS_Puff`) false)
    (`self.TurnOnButton`)
    (`KismetSystemLibrary.Delay` 0.5)
    (`SceneComponent.SetHiddenInGame` (`self.SM_Portalv3`) false false)
    (`SceneComponent.SetHiddenInGame` (`self.SM_Portalv2`) false false)
    (`KismetSystemLibrary.Delay` (`self.TimeToDisappear`))
    (`self.TurnOffButton`)
    (`ActorComponent.Activate` (`self.NS_Puff`) false)
    (`SceneComponent.SetHiddenInGame` (`self.SM_Portalv3`) true false)
    (`SceneComponent.SetHiddenInGame` (`self.SM_Portalv2`) true false)
    (set `self.isActive` false)))

(event `self.BoxCollision.OnComponentBeginOverlap`
  (params (OverlappedComponent :type "PrimitiveComponent Object Reference") (OtherActor :type "Actor Object Reference") (OtherComp :type "PrimitiveComponent Object Reference") (OtherBodyIndex :type Integer) (bFromSweep :type Boolean) (SweepResult :type "HitResult Structure (by ref)"))
  (if (`self.isActive`)
    (`KismetSystemLibrary.Delay` 0.5)
    (`KismetSystemLibrary.QuitGame` null "Quit")))

(event `TurnOnButton`
  (bind (_btnstartinglocation_x _btnstartinglocation_y _btnstartinglocation_z) (`KismetMathLibrary.BreakVector` (`self.BtnStartingLocation`)))
  (`ActorComponent.Activate` (`self.Niagara`) true)
  (`MaterialInstanceDynamic.SetScalarParameterValue` (`self.ButtonEmissiveMat`) (`self.NameEmissive`) 0.0)
  (bind (_direction _alpha) (`Timeline|Timeline` :!via `PlayFromStart` :!label _label)
    (:`Update`
      (`SceneComponent.K2_SetRelativeLocation` (`self.Button`) (`KismetMathLibrary.MakeVector` _btnstartinglocation_x (+ (`KismetMathLibrary.Lerp` 0.0 -5.0 _alpha) _btnstartinglocation_y) _btnstartinglocation_z) false false))))

(event `TurnOffButton`
  (`MaterialInstanceDynamic.SetScalarParameterValue` (`self.ButtonEmissiveMat`) (`self.NameEmissive`) (`self.BtnEmissiveIntensity`))
  (goto _label :!via `ReverseFromEnd`))

(fn `CanInteract`
  (params (Interactor :type "Interactor Interface (by ref)") (InteractionMethod :type "EInteractionMethod Enum" :default "KeyPress"))
  (returns (ReturnValue :type Boolean))
  (return false))

(fn `UserConstructionScript`)
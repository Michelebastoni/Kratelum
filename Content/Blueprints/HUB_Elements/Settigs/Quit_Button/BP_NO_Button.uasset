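; The "No" button of the hub's quit prompt, an interactable cube that grows in through a timeline-driven scale when spawned.
; Interact notifies BP_Yes_Button through YESQuitting and reverses the timeline to scale the cube back.
; Once IsQuitting is set, timeline updates trigger a delayed self-destroy.
; CanInteract always returns false, although Interact is implemented.
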(event `self.ReceiveBeginPlay`
  (bind (_direction _no_button) (`Timeline|Timeline` :!label _label)
    (:`Update`
      (`SceneComponent.SetWorldScale3D` (`self.Cube`) (`KismetMathLibrary.MakeVector` (* _no_button (`self.X_Scale`)) (* _no_button (`self.Y_Scale`)) (* _no_button (`self.Z_Scale`))))
      (if (`self.IsQuitting`)
        (`KismetSystemLibrary.Delay` 1.0)
        (`self.K2_DestroyActor`)))))

(event `self.Interact`
  (params (Interactor :type "Interactor Interface (by ref)") (InteractionMethod :type "EInteractionMethod Enum" :default "KeyPress"))
  (set `self.IsQuitting` true)
  (bind _returnvalue (`GameplayStatics.GetActorOfClass` "/Game/Blueprints/HUB_Elements/Settigs/Quit_Button/BP_Yes_Button.BP_Yes_Button_C"))
  (`/Game/Blueprints/HUB_Elements/Settigs/Quit_Button/BP_Yes_Button.YES_Quitting` _returnvalue)
  (goto _label :!via `Reverse`))

(fn `CanInteract`
  (params (Interactor :type "Interactor Interface (by ref)") (InteractionMethod :type "EInteractionMethod Enum" :default "KeyPress"))
  (returns (ReturnValue :type Boolean))
  (return false))

(fn `UserConstructionScript`)
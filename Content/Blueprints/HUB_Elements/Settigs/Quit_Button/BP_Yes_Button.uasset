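; BP_Yes_Button is the HUB "Yes" button for quitting, and its Interact event quits the game.
; On BeginPlay, a timeline animates the Cube's scale through per-axis multipliers.
; YES_Quitting flags the button and reverses that timeline, whose update then destroys the actor after a short delay.
; CanInteract always returns false as written.
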(event `self.ReceiveBeginPlay`
  (bind (_direction _yes_button) (`Timeline|T_YES Button` :!label _label)
    (:`Update`
      (`SceneComponent.SetWorldScale3D` (`self.Cube`) (`KismetMathLibrary.MakeVector` (* _yes_button (`self.X Scale`)) (* _yes_button (`self.Y Scale`)) (* _yes_button (`self.Z Scale`))))
      (if (`self.IsQuitting`)
        (`KismetSystemLibrary.Delay` 1.0)
        (`self.K2_DestroyActor`)))))

(event `YES_Quitting`
  (set `self.IsQuitting` true)
  (goto _label :!via `Reverse`))

(event `self.Interact`
  (params (Interactor :type "Interactor Interface (by ref)") (InteractionMethod :type "EInteractionMethod Enum" :default "KeyPress"))
  (`KismetSystemLibrary.QuitGame` null "Quit"))

(fn `CanInteract`
  (params (Interactor :type "Interactor Interface (by ref)") (InteractionMethod :type "EInteractionMethod Enum" :default "KeyPress"))
  (returns (ReturnValue :type Boolean))
  (return false))

(fn `UserConstructionScript`)
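; Sound icon for a settings sign button in the hub, which can light up to show a selected state.
; On BeginPlay it creates a dynamic material instance on the icon mesh, sets the Icon texture and starts unlit.
; ToggleEmissive recreates a missing material, then either resets the glow or schedules a next-tick callback, presumably LigthOn, which applies the selected emissive color and strength.
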(event `self.ReceiveBeginPlay`
  (`self.InitializeMaterials`))

(fn `InitializeMaterials`
  (bind _sm_nosound_icon (`self.SM_NoSound_Icon`))
  (bind _returnvalue (`PrimitiveComponent.CreateDynamicMaterialInstance` _sm_nosound_icon 0 "/Game/Materials/HUB_Material/M_Setting/M_Sound_Icon_Inst.M_Sound_Icon_Inst" "None"))
  (bind _output_get (set `self.IconMaterial` _returnvalue))
  (`PrimitiveComponent.SetMaterial` _sm_nosound_icon 0 _output_get)
  (`MaterialInstanceDynamic.SetTextureParameterValue` _output_get "Image" (`self.Icon`))
  (`MaterialInstanceDynamic.SetScalarParameterValue` _output_get "EmissiveStrength" 0.0)
  (`MaterialInstanceDynamic.SetVectorParameterValue` _output_get "EmissiveColor" (struct :`R` 1.0 :`G` 1.0 :`B` 1.0 :`A` 1.0)))

(fn `LigthOn`
  (bind _iconmaterial (`self.IconMaterial`))
  (`MaterialInstanceDynamic.SetScalarParameterValue` _iconmaterial "EmissiveStrength" (`self.SelectedEmissiveStrength`))
  (`MaterialInstanceDynamic.SetVectorParameterValue` _iconmaterial "EmissiveColor" (`self.EmissiveColor`)))

(fn `ToggleEmissive`
  (params (IsSelected :type Boolean))
  (bind _iconmaterial (`self.IconMaterial`))
  (`/Engine/EditorBlueprintResources/StandardMacros.IsValid` (`self.IconMaterial`)
    (:`Is Valid`
      _)
    (:`Is Not Valid`
      (`self.InitializeMaterials`)))
  (if IsSelected
    (`KismetSystemLibrary.K2_SetTimerForNextTickDelegate` (`|CreateDelegate` :!event `LigthOn`))
    (else
      (`MaterialInstanceDynamic.SetScalarParameterValue` _iconmaterial "EmissiveStrength" 0.0)
      (`MaterialInstanceDynamic.SetVectorParameterValue` _iconmaterial "EmissiveColor" (struct :`R` 1.0 :`G` 1.0 :`B` 1.0 :`A` 1.0)))))

(fn `UserConstructionScript`)
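; Moving target actor in the hub's settings elements that shuttles its Target component back and forth between points A and B.
; On BeginPlay it snaps Target to the starting endpoint chosen by GoToB.
; The Patrol timeline lerps its relative location to the opposite point, with play rate set to the inverse of MoovingTime.
; When each leg finishes, it flips GoToB and calls Move again, looping endlessly without Tick.
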(event `self.ReceiveBeginPlay`
  (`SceneComponent.K2_SetRelativeLocation` (`self.Target`) (select `bool` (`self.GoToB`) :`false` (`SceneComponent.RelativeLocation` (`self.B`)) :`true` (`SceneComponent.RelativeLocation` (`self.A`))) false true)
  (`self.Move`))

(event `Move`
  (`TimelineComponent.SetPlayRate` (`self.Patrol`) (/ 1.0 (`self.MoovingTime`)))
  (set `self.Relative Location` (`SceneComponent.RelativeLocation` (`self.Target`)))
  (bind (_direction _patrol) (`Timeline|Patrol` :!via `PlayFromStart`)
    (:`Update`
      (`SceneComponent.K2_SetRelativeLocation` (`self.Target`) (`KismetMathLibrary.VLerp` (`self.Relative Location`) (select `bool` (`self.GoToB`) :`false` (`SceneComponent.RelativeLocation` (`self.A`)) :`true` (`SceneComponent.RelativeLocation` (`self.B`))) _patrol) false false))
    (:`Finished`
      (set `self.GoToB` (not (`self.GoToB`)))
      (`self.Move`))))

(fn `UserConstructionScript`)
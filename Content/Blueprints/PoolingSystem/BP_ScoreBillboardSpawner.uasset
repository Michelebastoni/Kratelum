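; Pool-based spawner that shows death score billboards where enemies die.
; On BeginPlay it initializes itself and binds to the NPC subsystem's enemy-died event.
; Each death pulls a BP_DeathScoreBillboard from the pool, activates it with the killer, then teleports it to the enemy's location plus a spawn offset.
; The event's kill points are not passed to the billboard.
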(event `self.ReceiveBeginPlay`
  (`self.Init`)
  (add `NPCSubsystem.OnEnemyDied` (subsystem `NPCSubsystem`) (delegate `OnEnemyDied_Event`)))

(event `OnEnemyDied_Event`
  (params (KilledEnemy :type "Actor Object Reference") (KillPoints :type Integer) (Killer :type "Actor Object Reference"))
  (bind _returnvalue (`self.TryGetPoolable`))
  (bind _asbp_death_score_billboard (cast `/Game/Blueprints/Cosmetics/BP_DeathScoreBillboard` _returnvalue))
  (`/Game/Blueprints/Cosmetics/BP_DeathScoreBillboard.Toggle` _asbp_death_score_billboard Killer true)
  (`self.K2_SetActorLocation` _asbp_death_score_billboard (+ (`self.K2_GetActorLocation` KilledEnemy) (`self.SpawnOffset`)) false true))

(fn `UserConstructionScript`)
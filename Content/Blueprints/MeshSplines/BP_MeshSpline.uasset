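; Spline actor that tiles a static mesh along its path and can temporarily swap its material, apparently as trap feedback.
; The construction script adds fixed-length spline mesh segments with clamped tangents and configurable collision, with FullLength including the final partial section.
; AllowScaling instead only derives section length from actor X scale, without building segments.
; ChangeSplineMaterial swaps every segment's material, then calls itself after TrapTime to restore the normal one.
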(event `ChangeSplineMaterial`
  (params (Reset :type Boolean))
  (for _array_element (`self.SplineArray`)
    (`PrimitiveComponent.SetMaterial` _array_element 0 (select `bool` Reset :`false` (`self.MaterialToChange`) :`true` (`self.NormalMaterial`))))
  (if (not Reset)
    (`KismetSystemLibrary.Delay` (`self.TrapTime`))
    (`self.ChangeSplineMaterial` true)))

(fn `EndPosition`
  (params (Index :type Integer))
  (returns (Position :type "Vector Structure") (Tangent :type "Vector Structure"))
  (bind _spline (`self.Spline`))
  (bind _returnvalue (* (+ Index 1) (`self.SectionLength`)))
  (return (`SplineComponent.GetLocationAtDistanceAlongSpline` _spline _returnvalue "Local") (`KismetMathLibrary.ClampVectorSize` (`SplineComponent.GetTangentAtDistanceAlongSpline` _spline _returnvalue "Local") 0.0 (`self.SectionLength`))))

(fn `StartPosition`
  (params (Index :type Integer))
  (returns (Position :type "Vector Structure") (Tangent :type "Vector Structure"))
  (bind _spline (`self.Spline`))
  (bind _returnvalue (* Index (`self.SectionLength`)))
  (return (`SplineComponent.GetLocationAtDistanceAlongSpline` _spline _returnvalue "Local") (`KismetMathLibrary.ClampVectorSize` (`SplineComponent.GetTangentAtDistanceAlongSpline` _spline _returnvalue "Local") 0.0 (`self.SectionLength`))))

(fn `UserConstructionScript`
  (bind _returnvalue_x (`KismetMathLibrary.BreakVector` (`self.GetActorScale3D`)))
  (bind _loopindex (`self.LoopIndex`))
  (if (`self.AllowScaling`)
    (set `self.SectionLength` (* _returnvalue_x 100.0))
    (elif (`self.FullLength`)
      (for _index (range (+ (`KismetMathLibrary.FTrunc` (/ (`SplineComponent.GetSplineLength` (`self.Spline`)) (`self.SectionLength`))) 1))
        (set `self.LoopIndex` _index)
        (bind _returnvalue (`AddComponent|NODE_AddSplineMeshComponent-0` :!label _label))
        (`KismetArrayLibrary.Array_Add` (`self.SplineArray`) _returnvalue)
        (`StaticMeshComponent.SetStaticMesh` _returnvalue (`self.SplineMesh`))
        (`PrimitiveComponent.SetMaterial` _returnvalue 0 (`self.NormalMaterial`))
        (`SplineMeshComponent.SetForwardAxis` _returnvalue "X" true)
        (bind (_position _tangent) (`self.StartPosition` _loopindex))
        (bind (_position_2 _tangent_2) (`self.EndPosition` _loopindex))
        (`SplineMeshComponent.SetStartAndEnd` _returnvalue _position _tangent _position_2 _tangent_2 true)
        (`PrimitiveComponent.SetCollisionEnabled` _returnvalue (`self.CollysionType`)))
      (else
        (for _index_2 (range (`KismetMathLibrary.FTrunc` (/ (`SplineComponent.GetSplineLength` (`self.Spline`)) (`self.SectionLength`))))
          (set `self.LoopIndex` _index_2)
          (goto _label))))))
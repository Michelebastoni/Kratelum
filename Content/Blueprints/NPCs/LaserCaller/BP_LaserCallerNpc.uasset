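; Laser Caller NPC that can show an on-screen targeting marker tracking it for the player.
; On BeginPlay it optionally creates the targeting widget, and a timeline spins its cylinder while driving the emissive parameter.
; The enemy pooled delegate sets widget animation and re-enables tick, which projects the actor's location against viewport bounds to update marker visibility.
; IntegrityComponent death stops marker animation and tick.
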(event `self.ReceiveBeginPlay`
  (bind _returnvalue (`GameplayStatics.GetPlayerController` 0))
  (`|ExecutionSequence`
    (:`then_0`
      (if (`self.UseHelperMarker`)
        (bind _returnvalue_2 (`|CreateWidget` "/Game/Blueprints/Widgets/TargetingWidget/BPW_TargetingWidget.BPW_TargetingWidget_C" _returnvalue))
        (set `self.PlayerCtrl` _returnvalue)
        (set `self.MarkerWidget` _returnvalue_2)
        (`UserWidget.AddToViewport` _returnvalue_2 0)
        (`/Game/Blueprints/Widgets/TargetingWidget/BPW_TargetingWidget.SetTarget` _returnvalue_2 self)
        (add `self.OnEnemyPooledDelegate` (delegate `OnEnemyPooled_Event`))
        (`self.SetActorTickEnabled` false)))
    (:`then_1`
      (bind (_direction _newtrack_0) (`Timeline|Timeline`)
        (:`Update`
          (`SceneComponent.K2_AddLocalRotation` (`self.Cylinder`) (`KismetMathLibrary.MakeRotator` 0.0 15.0) false false)
          (`MeshComponent.SetScalarParameterValueOnMaterials` (`self.Cylinder`) "Emissive" (* _newtrack_0 5.0)))))))

(event `OnEnemyPooled_Event` :!signature `self.OnEnemyPooledDelegate`
  (params (bIsActive :type Boolean))
  (`/Game/Blueprints/Widgets/TargetingWidget/BPW_TargetingWidget.SetCanAnimate` (stale `self.ReceiveBeginPlay` _returnvalue_2) bIsActive)
  (`self.SetActorTickEnabled` true))

(event `self.ReceiveTick`
  (params (DeltaSeconds :type "Float (single-precision)"))
  (if (`self.UseHelperMarker`)
    (bind _returnvalue (`self.IsInViewport`))
    (if (not (and (`self.WasVisible`) _returnvalue))
      (bind _output_get (set `self.WasVisible` _returnvalue))
      (`/Game/Blueprints/Widgets/TargetingWidget/BPW_TargetingWidget.UpdateMarkerVisibility` (`self.MarkerWidget`) self _output_get))))

(event `self.integrityComponent.OnDeath`
  (params (owner :type "Actor Object Reference") (harmer :type "Actor Object Reference") (integrityComp :type "Integrity Object Reference") (currentIntegrityValue :type "Float (single-precision)"))
  (`/Game/Blueprints/Widgets/TargetingWidget/BPW_TargetingWidget.SetCanAnimate` (`self.MarkerWidget`) false)
  (`self.SetActorTickEnabled` false))

(fn `IsInViewport`
  (returns (ReturnValue :type Boolean))
  (bind (_returnvalue_x _returnvalue_y) (`KismetMathLibrary.BreakVector2D` (`WidgetLayoutLibrary.GetViewportSize`)))
  (bind _screenlocation (`PlayerController.ProjectWorldLocationToScreen` (`self.PlayerCtrl`) (`self.K2_GetActorLocation`) false))
  (return (and (> (`KismetMathLibrary.BreakVector2D` _screenlocation) 0.0) (> (`.Y` (`KismetMathLibrary.BreakVector2D` _screenlocation)) 0.0) (< (`KismetMathLibrary.BreakVector2D` _screenlocation) _returnvalue_x) (< (`.Y` (`KismetMathLibrary.BreakVector2D` _screenlocation)) _returnvalue_y))))

(fn `UserConstructionScript`)
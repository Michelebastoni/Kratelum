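; Kamikaze NPC Blueprint that handles barrel glow and explosion camera shake feedback on top of its parent class.
; A dynamic material instance caches the barrel's emissive strength and starts it dark.
; The AI controller's detonation delegate sets the detonating and animating flags, switching the glow on or off.
; The explosion delegate plays a strong or weak shake on the player controller, cached at player spawn, depending on whether the player was hit.
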(event `self.ReceiveBeginPlay`
  (`parent.ReceiveBeginPlay`)
  (bind _returnvalue (`PrimitiveComponent.CreateDynamicMaterialInstance` (`self.Barrel`) 0 "/Game/Models/Skeletal/Characters/Enemies/KAMIKAZE/EXPLOSIVES/M_KamikazeBarrel_Inst.M_KamikazeBarrel_Inst" "None"))
  (bind _output_get (set `self.BarrelMaterial` _returnvalue))
  (bind _returnvalue_2 (`MaterialInstanceDynamic.K2_GetScalarParameterValue` _output_get "EmissiveStrength"))
  (set `self.BarrelEmissive` _returnvalue_2)
  (`MaterialInstanceDynamic.SetScalarParameterValue` _output_get "EmissiveStrength" 0.0)
  (bind _asbp_kamikaze_npc_controller (cast `/Game/Blueprints/NPCs/Kamikaze/BP_KamikazeNpcController` (`self.GetController`)))
  (add `KamikazeNpcController.OnDetonationValueChangedDelegate` _asbp_kamikaze_npc_controller (`|CreateDelegate` :!event `OnDetonationValueChanged_Event`))
  (add `NPCSubsystem.OnPlayerSpawned` (subsystem `NPCSubsystem`) (delegate `OnPlayer_Spawned_Event`))
  (add `self.OnPlayerHitByExplosionDelegate` (delegate `OnPlayerHitByExplosion_Event`)))

(event `OnPlayer_Spawned_Event`
  (params (Player :type "PlayerCharacter Object Reference"))
  (set `self.PlayerTarget` Player)
  (set `self.PlayerCtrl` (`GameplayStatics.GetPlayerController` 0)))

(event `OnPlayerHitByExplosion_Event` :!signature `self.OnPlayerHitByExplosionDelegate`
  (params (bHasHitPlayer :type Boolean))
  (bind _playerctrl (`self.PlayerCtrl`))
  (if bHasHitPlayer
    (`/Game/Blueprints/Cosmetics/CameraShakeClasses/BP_CameraShaker.StrongCameraShake` _playerctrl)
    (else
      (`/Game/Blueprints/Cosmetics/CameraShakeClasses/BP_CameraShaker.WeakCameraShake` _playerctrl))))

(event `OnDetonationValueChanged_Event`
  (params (bIsDetonating :type Boolean))
  (bind _output_get (set `self.IsDetonating` bIsDetonating))
  (set `self.IsAnimating` _output_get)
  (`self.ToggleBarrelEmissive`))

(fn `ToggleBarrelEmissive`
  (bind _barrelmaterial (`self.BarrelMaterial`))
  (if (`self.IsAnimating`)
    (`MaterialInstanceDynamic.SetScalarParameterValue` _barrelmaterial "EmissiveStrength" (`self.BarrelEmissive`))
    (else
      (`MaterialInstanceDynamic.SetScalarParameterValue` _barrelmaterial "EmissiveStrength" 0.0))))

(fn `UserConstructionScript`)
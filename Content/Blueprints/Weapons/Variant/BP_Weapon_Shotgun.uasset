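; Shotgun weapon variant that drives a laser effect from its muzzle.
; On BeginPlay it moves the laser to the muzzle and caches the SteveJr reference.
; Each tick it traces from the muzzle along Steve's forward vector on the Camera channel.
; The hit point, or trace end on a miss, feeds the laser's vector parameter, which is named BeamWidth despite receiving a position.
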(event `self.ReceiveBeginPlay`
  (`SceneComponent.K2_SetWorldLocation` (`self.Laser`) (`self.GetMuzzleLocation`) false false)
  (set `self.Steve` (`/Game/Blueprints/RnD/BPFunctionsLibrary.GetSteveJr`)))

(event `self.ReceiveTick`
  (params (DeltaSeconds :type "Float (single-precision)"))
  (bind _returnvalue (`self.GetMuzzleLocation`))
  (bind _outhit (`KismetSystemLibrary.LineTraceSingle` :`Start` _returnvalue :`End` (+ _returnvalue (* (`SceneComponent.GetForwardVector` (`Actor.RootComponent` (`self.Steve`))) 9000.0)) :`TraceChannel` "TraceTypeQuery2" :`TraceColor` (struct :`R` 1.0 :`G` 1.0 :`B` 1.0) :`TraceHitColor` (struct) :`DrawTime` 0.0))
  (bind (_bblockinghit _binitialoverlap _time _distance _location _impactpoint _normal _impactnormal _physmat _hitactor _hitcomponent _hitbonename _bonename _hititem _elementindex _faceindex _tracestart _traceend) (`GameplayStatics.BreakHitResult` _outhit))
  (`FXSystemComponent.SetVectorParameter` (`self.Laser`) "BeamWidth" (`KismetMathLibrary.SelectVector` _impactpoint _traceend _bblockinghit)))

(fn `UserConstructionScript`)
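; BP_Party_Weapon is a weapon whose party music plays only while it is being fired.
; BeginPlay creates a 2D sound, starts it at an initial time and pauses it immediately; each shot unpauses it or restarts it if not playing.
; A Tick-driven 0.2-second Delay polls and clears an IsShooting flag, pausing the music when no shot has set it.
; Destroying the weapon stops the sound.
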(event `self.ReceiveBeginPlay`
  ;[0 0 0] PARTY LOGIC (Pls Dont touch)
  (bind _returnvalue (`GameplayStatics.CreateSound2D` (`self.PartySound`) 1.0 1.0 0.0 null false false))
  (bind _output_get (set `self.PartySoundComp` _returnvalue))
  (`AudioComponent.Play` _output_get (`self.InitialPartySoundTime`))
  (`AudioComponent.SetPaused` _output_get true)
  (add `self.onShoot` (delegate `onShoot_Event`))
  (add `self.OnDestroyed` (delegate `OnDestroyed_Event`)))

(event `OnDestroyed_Event` :!signature `self.OnDestroyed`
  (params (DestroyedActor :type "Actor Object Reference"))
  ;[0 0 0] PARTY LOGIC (Pls Dont touch)
  (`AudioComponent.Stop` (`self.PartySoundComp`)))

(event `onShoot_Event` :!signature `self.onShoot`
  (params (bullets :type Integer))
  (bind _partysoundcomp (`self.PartySoundComp`))
  ;[0 0 0] PARTY LOGIC (Pls Dont touch)
  (if (`AudioComponent.IsPlaying` _partysoundcomp)
    (`AudioComponent.SetPaused` _partysoundcomp false)
    (set `self.bIsShooting` true)
    (else
      (`AudioComponent.Play` _partysoundcomp (`self.InitialPartySoundTime`)))))

(event `self.ReceiveTick`
  (params (DeltaSeconds :type "Float (single-precision)"))
  (bind _partysoundcomp (`self.PartySoundComp`))
  ;[0 0 0] PARTY LOGIC (Pls Dont touch)
  (`KismetSystemLibrary.Delay` 0.2)
  (if (`self.bIsShooting`)
    (set `self.bIsShooting` false)
    (elif (`AudioComponent.IsPlaying` _partysoundcomp)
      (`AudioComponent.SetPaused` _partysoundcomp true))))

(fn `UserConstructionScript`)
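; Cosmetic director that plays a lightning-and-thunder effect whenever a game phase completes.
; It keeps its DirectionalLight hidden from construction and BeginPlay, and binds to the phase-completed delegate on play.
; Each completion flickers the light on and off through a hard-coded chain of short random delays, then plays a 2D thunder cue and switches the light off, ignoring the phase parameters.
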(event `self.ReceiveBeginPlay`
  (add `self.OnPhaseCompletedDelegate` (delegate `OnPhaseCompleted_Event`))
  (`SceneComponent.SetHiddenInGame` (`self.DirectionalLight`) true false)
  (`SceneComponent.SetVisibility` (`self.DirectionalLight`) false false))

(event `OnPhaseCompleted_Event` :!signature `self.OnPhaseCompletedDelegate`
  (params (PreviousPhase :type "EnemyPhaseData Object Reference") (CurrentPhase :type "EnemyPhaseData Object Reference") (PhaseIndex :type Integer) (IsLastPhase :type Boolean))
  (bind _returnvalue (`KismetMathLibrary.RandomFloatInRange` 0.1 0.3))
  (bind _directionallight (`self.DirectionalLight`))
  (bind _directionallight_2 (`self.DirectionalLight`))
  (`SceneComponent.SetVisibility` (`self.DirectionalLight`) true false)
  (`SceneComponent.SetHiddenInGame` _directionallight_2 false false)
  (`KismetSystemLibrary.Delay` _returnvalue)
  (`SceneComponent.SetHiddenInGame` _directionallight_2 true false)
  (`KismetSystemLibrary.Delay` _returnvalue)
  (`SceneComponent.SetHiddenInGame` _directionallight_2 false false)
  (`KismetSystemLibrary.Delay` _returnvalue)
  (`SceneComponent.SetHiddenInGame` _directionallight_2 true false)
  (`KismetSystemLibrary.Delay` _returnvalue)
  (`SceneComponent.SetHiddenInGame` _directionallight false false)
  (`KismetSystemLibrary.Delay` _returnvalue)
  (`SceneComponent.SetHiddenInGame` _directionallight true false)
  (`KismetSystemLibrary.Delay` _returnvalue)
  (`SceneComponent.SetHiddenInGame` _directionallight false false)
  (`KismetSystemLibrary.Delay` _returnvalue)
  (`SceneComponent.SetHiddenInGame` _directionallight true false)
  (`KismetSystemLibrary.Delay` _returnvalue)
  (`GameplayStatics.PlaySound2D` "/Game/Audio/SFX/0_Game/GameplayFeedbacks/ThunderStruck_Cue.ThunderStruck_Cue" 1.0 1.0 0.0 null null)
  (`SceneComponent.SetVisibility` (`self.DirectionalLight`) false false))

(fn `UserConstructionScript`
  (`SceneComponent.SetVisibility` (`self.DirectionalLight`) false false))
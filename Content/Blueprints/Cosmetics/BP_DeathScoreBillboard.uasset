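; Pooled cosmetic billboard that pops up on a death, with an extra trap billboard when the killer is a trap other than the orbital laser.
; Toggle shows or hides the billboards based on the killer.
; When pooled out, a timeline animates the death billboard's height, then after a time-to-live delay it returns itself to the pool.
; An animating flag reports whether it is in use.
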(event `self.Initialize`
  (params (Pool :type "Pool Object Reference"))
  (set `self.Pool` Pool)
  (`self.Toggle` null)
  (set `self.IsAnimating` false))

(event `self.OnObjectPooled`
  (set `self.IsAnimating` true)
  (bind (_direction _death_number) (`Timeline|DeathNumberAnimation` :!via `PlayFromStart`)
    (:`Update`
      (`SceneComponent.K2_SetRelativeLocation` (`self.DeathBillboard`) (`KismetMathLibrary.MakeVector` 0.0 0.0 (* _death_number (`self.ZOffsetMultiplier`))) false false))
    (:`Finished`
      (`KismetSystemLibrary.Delay` (`self.TimeToLive`))
      (`Pool.ReturnPoolable` (`self.Pool`) self))))

(event `self.OnObjectReturnToPool`
  (`self.Toggle` null)
  (set `self.IsAnimating` false))

(fn `GetIsInUse`
  (returns (ReturnValue :type Boolean))
  (return (`self.IsAnimating`)))

(fn `Toggle`
  (params (Killer :type "Actor Object Reference") (Activate :type Boolean))
  (if Activate
    (`SceneComponent.SetHiddenInGame` (`self.DeathBillboard`) false false)
    (if (and (`GameplayStatics.ObjectIsA` Killer "/Script/TBO02.Trap") (not (`GameplayStatics.ObjectIsA` Killer "/Game/Blueprints/Arena_Prototyping/Traps/BP_Trap_OrbitalLaser.BP_Trap_OrbitalLaser_C")))
      (`SceneComponent.SetHiddenInGame` (`self.TrapDeathBillboard`) false false))
    (else
      (`SceneComponent.SetHiddenInGame` (`self.TrapDeathBillboard`) true false)
      (`SceneComponent.SetHiddenInGame` (`self.DeathBillboard`) true false))))

(fn `UserConstructionScript`)
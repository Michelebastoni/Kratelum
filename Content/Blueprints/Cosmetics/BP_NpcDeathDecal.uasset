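; BP_NpcDeathDecal is a pooled cosmetic actor for NPC death decals that vanishes after a set time.
; Initialize stores the owning pool and starts the decal hidden and unplaced.
; When pooled out, it becomes visible, waits TimeToVanish, then returns itself to the pool, which hides it again.
; An IsPlaced flag tracks this state and is exposed through GetIsInUse.
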(event `self.Initialize`
  (params (Pool :type "Pool Object Reference"))
  (set `self.Pool` Pool)
  (`self.SetActorHiddenInGame` true)
  (set `self.IsPlaced` false))

(event `self.OnObjectPooled`
  (set `self.IsPlaced` true)
  (`self.SetActorHiddenInGame` false)
  (`KismetSystemLibrary.Delay` (`self.TimeToVanish`))
  (`Pool.ReturnPoolable` (`self.Pool`) self))

(event `self.OnObjectReturnToPool`
  (`self.SetActorHiddenInGame` true)
  (set `self.IsPlaced` false))

(fn `GetIsInUse`
  (returns (ReturnValue :type Boolean))
  (return (`self.IsPlaced`)))

(fn `UserConstructionScript`)
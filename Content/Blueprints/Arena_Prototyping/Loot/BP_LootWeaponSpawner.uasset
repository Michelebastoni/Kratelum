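; Arena loot spawner that periodically spawns a weapon pickup at a target point tagged "WeaponTarget", keeping one active at a time.
; A looping timer runs Spawner, which picks a point and a weighted-random weapon variant only when no current weapon exists.
; An existing weapon is destroyed and respawned from the previous pick.
; UpdateTargetPoints refreshes the point list, and StopSpawner disables spawning and removes the current weapon.
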(event `self.ReceiveBeginPlay`
  (bind _returnvalue (`KismetSystemLibrary.K2_SetTimerDelegate` (delegate `Spawner`) (`self.LootTimer`) true))
  (set `self.LootTimerValue` _returnvalue))

(event `Spawner`
  (bind _spawntargetpoint (`self.SpawnTargetPoint`))
  (bind _currentweapon (`self.CurrentWeapon`))
  (if (`self.bCanSpawn`)
    (`/Engine/EditorBlueprintResources/StandardMacros.IsValid` _currentweapon
      (:`Is Valid`
        (`self.K2_DestroyActor` _currentweapon))
      (:`Is Not Valid`
        (bind _output_get (set `self.LocalItem` (`|GetArrayItem` _spawntargetpoint (`KismetMathLibrary.RandomInteger` (`KismetArrayLibrary.Array_LastIndex` _spawntargetpoint)))))
        (bind _returnvalue (`FunctionLibrary.WeightedExtraction` (`self.WeaponVariants`)))
        (bind _asbp_basepup_weapon (castclass `/Game/Blueprints/Arena_Prototyping/WeaponVariant/BP_BASEPUpWeapon` _returnvalue))))
    (bind _output_get_2 (set `self.RandomWeaponToSpawn` _asbp_basepup_weapon))
    (bind _returnvalue_2 (`|SpawnActorFromClass` _output_get_2 (`KismetMathLibrary.MakeTransform` (`self.K2_GetActorLocation` _output_get)) "AdjustIfPossibleButAlwaysSpawn" "MultiplyWithRoot" null null))
    (set `self.CurrentWeapon` _returnvalue_2)))

(event `UpdateTargetPoints`
  (bind _outactors (`GameplayStatics.GetAllActorsOfClassWithTag` "/Script/Engine.TargetPoint" "WeaponTarget"))
  (set `self.SpawnTargetPoint` _outactors))

(fn `StopSpawner`
  (bind _currentweapon (`self.CurrentWeapon`))
  (set `self.bCanSpawn` false)
  (`/Engine/EditorBlueprintResources/StandardMacros.IsValid` _currentweapon
    (:`Is Valid`
      (`self.K2_DestroyActor` _currentweapon))))

(fn `UserConstructionScript`)
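; BP_LootPowerUpSpawner spawns one loot power-up at a time in the arena on a looping LootTimer.
; With no live power-up, it picks a random cached target point and a weighted-random BP_BASEPUp class.
; If one still exists, it replaces it using the previous class and point.
; UpdateTargetPoints caches points tagged PowerUpTarget, and StopSpawner disables spawning and destroys the current power-up.
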(event `self.ReceiveBeginPlay`
  (bind _returnvalue (`KismetSystemLibrary.K2_SetTimerDelegate` (delegate `Spawner`) (`self.LootTimer`) true))
  (set `self.LootTimerValue` _returnvalue))

(event `Spawner`
  (bind _spawntargetpoint (`self.SpawnTargetPoint`))
  (bind _currentpowerup (`self.CurrentPowerUp`))
  (if (`self.bCanSpawn`)
    (`/Engine/EditorBlueprintResources/StandardMacros.IsValid` _currentpowerup
      (:`Is Valid`
        (`self.K2_DestroyActor` _currentpowerup))
      (:`Is Not Valid`
        (bind _output_get (set `self.LocalItem` (`|GetArrayItem` _spawntargetpoint (`KismetMathLibrary.RandomInteger` (`KismetArrayLibrary.Array_LastIndex` _spawntargetpoint)))))
        (bind _returnvalue (`FunctionLibrary.WeightedExtraction` (`self.PowerUps`)))
        (bind _asbp_basepup (castclass `/Game/Blueprints/Arena_Prototyping/PowerUp/BP_BASEPUp` _returnvalue))))
    (bind _output_get_2 (set `self.RandomPowerUpToSpawn` _asbp_basepup))
    (bind _returnvalue_2 (`|SpawnActorFromClass` _output_get_2 (`KismetMathLibrary.MakeTransform` (`self.K2_GetActorLocation` _output_get)) "AdjustIfPossibleButAlwaysSpawn" "MultiplyWithRoot" null null))
    (set `self.CurrentPowerUp` _returnvalue_2)))

(event `UpdateTargetPoints`
  (bind _outactors (`GameplayStatics.GetAllActorsOfClassWithTag` "/Script/Engine.TargetPoint" "PowerUpTarget"))
  (set `self.SpawnTargetPoint` _outactors))

(fn `StopSpawner`
  (bind _currentpowerup (`self.CurrentPowerUp`))
  (set `self.bCanSpawn` false)
  (`/Engine/EditorBlueprintResources/StandardMacros.IsValid` _currentpowerup
    (:`Is Valid`
      (`self.K2_DestroyActor` _currentpowerup))))

(fn `UserConstructionScript`)
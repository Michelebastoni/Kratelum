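; Arena weapon-variant pickup for the SkullBreaker, which temporarily grants SteveJr a weapon variant using shotgun data.
; A timeline started on BeginPlay spins the weapon mesh around yaw.
; On sphere overlap with SteveJr, it grants the variant and plays a voice cue, or only spawns a Niagara effect if the ultimate is active.
; The actor destroys itself in both cases.
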(event `self.ReceiveBeginPlay`
  (`parent.ReceiveBeginPlay`)
  (`Timeline|Timeline` :!via `PlayFromStart`
    (:`Update`
      (`SceneComponent.K2_AddLocalRotation` (`self.WeaponMesh`) (`KismetMathLibrary.MakeRotator` 0.0 0.0 3.0) false false))))

(event `self.SphereCollision.OnComponentBeginOverlap`
  (params (OverlappedComponent :type "PrimitiveComponent Object Reference") (OtherActor :type "Actor Object Reference") (OtherComp :type "PrimitiveComponent Object Reference") (OtherBodyIndex :type Integer) (bFromSweep :type Boolean) (SweepResult :type "HitResult Structure (by ref)"))
  (bind _assteve_jr (cast `/Game/Blueprints/Character_Test/SteveJr` OtherActor))
  (if (`/Game/Blueprints/Character_Test/SteveJr.IsUltimateActive` _assteve_jr)
    (`NiagaraFunctionLibrary.SpawnSystemAtLocation` "/Game/VFX/Weapon_VFX/NS_QTEFirstCombo.NS_QTEFirstCombo" (`self.K2_GetActorLocation`))
    (else
      (`/Game/Blueprints/Character_Test/SteveJr.GainWeaponVariant` _assteve_jr (`self.Weapon Duration`) (`self.ShotgunData`))
      (`GameplayStatics.PlaySound2D` "/Game/Audio/SFX/0_Weapon/Weapon_Voice/SFX_SkullBreaker_Voice_Cue.SFX_SkullBreaker_Voice_Cue" 1.0 1.0 0.0 null null)))
  (`self.K2_DestroyActor`))

(fn `UserConstructionScript`
  (`parent.UserConstructionScript`))
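; BP_BASEPUpWeapon is a base pickup, apparently for weapons, that homes in on the player when SteveJr overlaps it.
; An optional despawn timer spawns a Niagara effect and destroys the actor, unless the overlap clears it first.
; On overlap, one timeline lerps it along the player's forward vector, then another lerps it to the player's live position.
; A half-second delay also forces that switch to homing.
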(event `self.ReceiveBeginPlay`
  (if (> (`self.DespawnTime`) 0.0)
    (bind _returnvalue (`KismetSystemLibrary.K2_SetTimerDelegate` (delegate `DestroyTimer`) (`self.DespawnTime`)))
    (set `self.TimerValue` _returnvalue)))

(event `DestroyTimer`
  (`NiagaraFunctionLibrary.SpawnSystemAtLocation` "/Game/VFX/Weapon_VFX/NS_QTEFirstCombo.NS_QTEFirstCombo" (`self.K2_GetActorLocation`))
  (`self.K2_DestroyActor`))

(event `self.AbsorptionCollision.OnComponentBeginOverlap`
  (params (OverlappedComponent :type "PrimitiveComponent Object Reference") (OtherActor :type "Actor Object Reference") (OtherComp :type "PrimitiveComponent Object Reference") (OtherBodyIndex :type Integer) (bFromSweep :type Boolean) (SweepResult :type "HitResult Structure (by ref)"))
  (cast `/Game/Blueprints/Character_Test/SteveJr` OtherActor)
  (`KismetSystemLibrary.K2_ClearAndInvalidateTimerHandle` (`self.TimerValue`))
  (set `self.PushAwayLocation` (+ (`self.K2_GetActorLocation`) (* (`KismetMathLibrary.GetForwardVector` (`self.K2_GetActorRotation` (`GameplayStatics.GetPlayerPawn` 0))) 250.0)))
  (`|ExecutionSequence`
    (:`then_0`
      (bind (_direction _value) (`Timeline|HomeAwayFromPlayer` :!via `PlayFromStart`)
        (:`Update`
          (`self.K2_SetActorLocation` (`KismetMathLibrary.VLerp` (`self.K2_GetActorLocation`) (`self.PushAwayLocation`) (* _value (`self.AnimationValue`)))))
        (:`Finished`
          (bind (_direction_2 _value_2) (`Timeline|HomeToPlayer` :!via `PlayFromStart` :!label _label)
            (:`Update`
              (`self.K2_SetActorLocation` (`KismetMathLibrary.VLerp` (`self.K2_GetActorLocation`) (`self.K2_GetActorLocation` (`GameplayStatics.GetPlayerPawn` 0)) (* _value_2 (`self.AnimationValue`)))))))))
    (:`then_1`
      (`KismetSystemLibrary.Delay` 0.5)
      (`TimelineComponent.Stop` (`self.HomeAwayFromPlayer`))
      (goto _label :!via `PlayFromStart`))))

(fn `UserConstructionScript`)
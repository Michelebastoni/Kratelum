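; BP_EESoulCollectible is a soul pickup that, once spawned, bursts outward and then flies to the game mode's SoulTarget.
; On BeginPlay it caches that target and lerps toward a point offset along the target's forward vector using a timeline.
; A parallel half-second delay stops HomeAwayFromPlayer and starts the homing timeline, which tracks the target's live location and destroys the actor when finished.
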(event `self.ReceiveBeginPlay`
  (bind (_asmy_gm _bsuccess) (cast `/Game/Blueprints/Character_Test/My_GM` (`GameplayStatics.GetGameMode`) :!pure true))
  (`KismetSystemLibrary.DelayUntilNextTick`)
  (if _bsuccess
    (bind _soultarget (`/Game/Blueprints/Character_Test/My_GM.SoulTarget` _asmy_gm)
      (:`then`
        (set `self.Target` _soultarget)
        (set `self.PushAwayLocation` (+ (`self.K2_GetActorLocation`) (* (`KismetMathLibrary.GetForwardVector` (`self.K2_GetActorRotation` (`self.Target`))) 250.0)))
        (`|ExecutionSequence`
          (:`then_0`
            (bind (_direction _value) (`Timeline|Timeline_1` :!via `PlayFromStart`)
              (:`Update`
                (`self.K2_SetActorLocation` (`KismetMathLibrary.VLerp` (`self.K2_GetActorLocation`) (`self.PushAwayLocation`) (* _value (`self.AnimationValue`)))))
              (:`Finished`
                (bind (_direction_2 _value_2) (`Timeline|Timeline_2` :!via `PlayFromStart` :!label _label)
                  (:`Update`
                    (`self.K2_SetActorLocation` (`KismetMathLibrary.VLerp` (`self.K2_GetActorLocation`) (`self.K2_GetActorLocation` (`self.Target`)) (* _value_2 (`self.AnimationValue`)))))
                  (:`Finished`
                    (`self.K2_DestroyActor`))))))
          (:`then_1`
            (`KismetSystemLibrary.Delay` 0.5)
            (`TimelineComponent.Stop` (`self.HomeAwayFromPlayer`))
            (goto _label :!via `PlayFromStart`))))
      (:`else`))))

(fn `UserConstructionScript`
  (`parent.UserConstructionScript`))
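; BP_PUpShieldProtection is a shield protection power-up pickup for the arena prototype.
; When a SteveJr overlaps its collision sphere, it plays a 2D voice cue, grants the power-up through GainPowerUp on that character, then destroys itself.
; The duration passed is ShieldDuration minus the character's FlickingDelay.
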(event `self.ReceiveBeginPlay`
  (`parent.ReceiveBeginPlay`))

(event `self.SphereCollison.OnComponentBeginOverlap`
  (params (OverlappedComponent :type "PrimitiveComponent Object Reference") (OtherActor :type "Actor Object Reference") (OtherComp :type "PrimitiveComponent Object Reference") (OtherBodyIndex :type Integer) (bFromSweep :type Boolean) (SweepResult :type "HitResult Structure (by ref)"))
  (bind _assteve_jr (cast `/Game/Blueprints/Character_Test/SteveJr` OtherActor))
  (`GameplayStatics.PlaySound2D` "/Game/Audio/SFX/0_PowerUp/Voice/SFX_ShieldProtection_Voice_Cue.SFX_ShieldProtection_Voice_Cue" 1.0 1.0 0.0 null null)
  (`/Game/Blueprints/Character_Test/SteveJr.GainPowerUp` _assteve_jr "NewEnumerator2" (- (`self.ShieldDuration`) (`/Game/Blueprints/Character_Test/SteveJr.FlickingDelay` _assteve_jr)) (`self.PowerUp_Name`))
  (`self.K2_DestroyActor`))

(fn `UserConstructionScript`
  (`parent.UserConstructionScript`))
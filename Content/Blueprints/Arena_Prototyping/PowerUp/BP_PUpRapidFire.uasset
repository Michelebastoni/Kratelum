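; BP_PUpRapidFire is an arena power-up pickup that grants rapid fire to the SteveJr character.
; On sphere overlap, an active weapon variant is re-granted with its current duration and data.
; If rapid fire is not already active, the weapon reloads, rapid fire increases and the HUD power-up sign shows the collectible.
; It then plays a 2D sound and destroys itself, even when no boost is applied.
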(event `self.SphereCollison.OnComponentBeginOverlap`
  (params (OverlappedComponent :type "PrimitiveComponent Object Reference") (OtherActor :type "Actor Object Reference") (OtherComp :type "PrimitiveComponent Object Reference") (OtherBodyIndex :type Integer) (bFromSweep :type Boolean) (SweepResult :type "HitResult Structure (by ref)"))
  (bind _assteve_jr (cast `/Game/Blueprints/Character_Test/SteveJr` OtherActor))
  (if (`/Game/Blueprints/Character_Test/SteveJr.IsWeaponVariantActive` _assteve_jr)
    (`/Game/Blueprints/Character_Test/SteveJr.GainWeaponVariant` _assteve_jr (`/Game/Blueprints/Character_Test/SteveJr.CurrentVariantDuration` _assteve_jr) (`/Game/Blueprints/Character_Test/SteveJr.CurrentWeaponData` _assteve_jr)))
  (if (not (`/Game/Blueprints/Character_Test/SteveJr.IsInRapidFire` _assteve_jr))
    (`Weapon.ApplyReload` (`GenericCharacter.GetCurrentWeapon` _assteve_jr))
    (`/Game/Blueprints/Character_Test/SteveJr.IncreaseRapidFire` _assteve_jr)
    (`/Game/Blueprints/Widgets/PowerUPSign_Widget/WBP_PowerUpSign.ShowCollectible` (`/Game/Blueprints/Widgets/BPW_HUD.WBP_PowerUpSign` (`/Game/Blueprints/Character_Test/SteveJr.HUD` _assteve_jr)) "NewEnumerator0" (`self.SignCollectible`)))
  (`GameplayStatics.PlaySound2D` (`self.Sound`) 1.0 1.0 0.0 null null)
  (`self.K2_DestroyActor`))

(fn `UserConstructionScript`
  (`parent.UserConstructionScript`))
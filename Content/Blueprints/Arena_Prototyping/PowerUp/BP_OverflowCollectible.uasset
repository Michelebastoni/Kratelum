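; BP_OverflowCollectible is an arena power-up pickup that grants overflow to the SteveJr character.
; When its collision sphere overlaps a SteveJr, it adds its overflow value to that character's Overflow component, unless the character's ultimate is active.
; The pickup destroys itself on any SteveJr contact, so it is still consumed without granting overflow during an active ultimate.
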(event `self.SphereCollison.OnComponentBeginOverlap`
  (params (OverlappedComponent :type "PrimitiveComponent Object Reference") (OtherActor :type "Actor Object Reference") (OtherComp :type "PrimitiveComponent Object Reference") (OtherBodyIndex :type Integer) (bFromSweep :type Boolean) (SweepResult :type "HitResult Structure (by ref)"))
  (bind _assteve_jr (cast `/Game/Blueprints/Character_Test/SteveJr` OtherActor))
  (if (not (`/Game/Blueprints/Character_Test/SteveJr.IsUltimateActive` _assteve_jr))
    (`Overflow.AddOverflow` (`PlayerCharacter.GetOverflowComponent` _assteve_jr) (`self.OverfrlowValue`)))
  (`self.K2_DestroyActor`))

(fn `UserConstructionScript`
  (`parent.UserConstructionScript`))
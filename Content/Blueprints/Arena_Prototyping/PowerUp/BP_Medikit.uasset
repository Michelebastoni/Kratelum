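; BP_Medikit is a health pickup that heals SteveJr and destroys itself.
; On sphere overlap it spawns an NS_HealingCross Niagara effect on SteveJr's mesh, or only destroys its stored effect if still valid.
; This effect step runs before the cast, so any overlapping actor triggers it.
; Only a SteveJr overlap adds HealValue through the Integrity component, plays a 2D sound and destroys the pickup.
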(event `self.ReceiveBeginPlay`
  (`parent.ReceiveBeginPlay`))

(event `self.SphereCollison.OnComponentBeginOverlap`
  (params (OverlappedComponent :type "PrimitiveComponent Object Reference") (OtherActor :type "Actor Object Reference") (OtherComp :type "PrimitiveComponent Object Reference") (OtherBodyIndex :type Integer) (bFromSweep :type Boolean) (SweepResult :type "HitResult Structure (by ref)"))
  (`self.NiagaraActive`
    (:`then`
      (`ActorComponent.K2_DestroyComponent` (`self.NiagaraActive`)))
    (:`else`
      (bind _returnvalue (`NiagaraFunctionLibrary.SpawnSystemAttached` "/Game/VFX/Level_VFX/Medikit/NS_HealingCross.NS_HealingCross" (`Character.Mesh` (`/Game/Blueprints/RnD/BPFunctionsLibrary.GetSteveJr`)) "None" (0.0 0.0 0.0) (struct) "KeepRelativeOffset" true))
      (set `self.NiagaraActive` _returnvalue)))
  (bind _assteve_jr (cast `/Game/Blueprints/Character_Test/SteveJr` OtherActor))
  (`Integrity.AddIntegrityValue` (`GenericCharacter.GetIntegrityComponent` _assteve_jr) (`self.HealValue`) self)
  (`GameplayStatics.PlaySound2D` (`self.Sound`) 1.0 1.0 0.0 null null)
  (`self.K2_DestroyActor`))

(fn `UserConstructionScript`
  (`parent.UserConstructionScript`))
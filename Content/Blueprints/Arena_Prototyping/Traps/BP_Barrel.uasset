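; Explosive barrel trap that takes damage through its Integrity component and detonates when that is depleted.
; On death, a timer and FlipFlop blink the barrel's emissive dynamic material for a set number of steps before the explosion effect and sound play.
; A sphere overlap then sends damage to nearby actors, plays a strong camera shake if the player is caught or a weak one otherwise, and the barrel is destroyed.
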(event `self.ReceiveBeginPlay`
  (`ActorComponent.Activate` (`self.NS_Puff`) false)
  (`self.InitBarrelMaterials`))

(event `self.Damage`
  (params (damageValue :type "Float (single-precision)") (harmer :type "Actor Object Reference"))
  (`Integrity.SubtractIntegrityValue` (`self.Integrity`) damageValue harmer))

(event `GlowingBarrel_Event`
  (`/Engine/EditorBlueprintResources/StandardMacros.FlipFlop`
    (:`A`
      (`MaterialInstanceDynamic.SetScalarParameterValue` (`self.EmissiveBarrelMaterial`) (`self.EmissiveParamName`) (`self.EmissiveStrength`)))
    (:`B`
      (`MaterialInstanceDynamic.SetScalarParameterValue` (`self.EmissiveBarrelMaterial`) (`self.EmissiveParamName`) 0.0))))

(event `self.Integrity.OnDeath`
  (params (owner :type "Actor Object Reference") (harmer :type "Actor Object Reference") (integrityComp :type "Integrity Object Reference") (currentIntegrityValue :type "Float (single-precision)"))
  (bind (_returnvalue_x _returnvalue_y _returnvalue_z) (`KismetMathLibrary.BreakVector` (`self.K2_GetActorLocation`)))
  (bind _returnvalue (`KismetSystemLibrary.K2_SetTimerDelegate` (delegate `GlowingBarrel_Event`) (`self.GlowingIntervalDelay`) true))
  (`KismetSystemLibrary.Delay` (+ (* (`self.GlowingSteps`) (`self.GlowingIntervalDelay`)) 0.1))
  (`KismetSystemLibrary.K2_ClearAndInvalidateTimerHandle` _returnvalue)
  (`NiagaraFunctionLibrary.SpawnSystemAtLocation` "/Game/VFX/Level_VFX/Traps/NS_ExplosionGroundBig.NS_ExplosionGroundBig" (`KismetMathLibrary.MakeVector` _returnvalue_x _returnvalue_y (+ _returnvalue_z 63.0)) (struct) (1.0 1.0 1.0) true true "AutoRelease")
  (`GameplayStatics.PlaySoundAtLocation` (`self.ExplosionSound`) (`self.K2_GetActorLocation`) (struct) 3.5 1.0 0.0 null null null null)
  (`self.MakeDamage`)
  (`self.K2_DestroyActor`))

(fn `InitBarrelMaterials`
  (bind _returnvalue (`PrimitiveComponent.CreateDynamicMaterialInstance` (`self.SM_Barrel`) 0 "/Game/Materials/Models/BarrelMaterial/M_GlowingBarrel_Inst.M_GlowingBarrel_Inst" "None"))
  (bind _output_get (set `self.EmissiveBarrelMaterial` _returnvalue))
  (bind _returnvalue_2 (`MaterialInstanceDynamic.K2_GetScalarParameterValue` _output_get (`self.EmissiveParamName`)))
  (set `self.EmissiveStrength` _returnvalue_2)
  (`MaterialInstanceDynamic.SetScalarParameterValue` _output_get (`self.EmissiveParamName`) 0.0))

(fn `MakeDamage`
  (bind _returnvalue (`GameplayStatics.GetPlayerController` 0))
  (bind (_returnvalue_x _returnvalue_y _returnvalue_z) (`KismetMathLibrary.BreakVector` (`self.K2_GetActorLocation`)))
  (bind _outactors (`KismetSystemLibrary.SphereOverlapActors` (`KismetMathLibrary.MakeVector` _returnvalue_x _returnvalue_y (+ _returnvalue_z 63.0)) (`self.Damage Radius`) (`|MakeArray` "ObjectTypeQuery3" "ObjectTypeQuery6" "ObjectTypeQuery2" "ObjectTypeQuery8" :!type "EObjectTypeQuery Enum") null (`|MakeArray` self :!type "Actor Object Reference")))
  (for _array_element _outactors
    (message `IntegrityHolder.Damage` _array_element (`self.BarrelDamage`) self)
    (if (not (`self.HasHitCharacter`))
      (set `self.HasHitCharacter` (`.bSuccess` (cast `PlayerCharacter` _array_element :!pure true)))))
  (if (`self.HasHitCharacter`)
    (`/Game/Blueprints/Cosmetics/CameraShakeClasses/BP_CameraShaker.StrongCameraShake` _returnvalue)
    (else
      (`/Game/Blueprints/Cosmetics/CameraShakeClasses/BP_CameraShaker.WeakCameraShake` _returnvalue)))
  (return))

(fn `UserConstructionScript`)
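; Tesla tower arena trap that, when toggled, zaps nearby pawns for a limited active duration.
; A timeline grows and shrinks a spark sphere sized to the damage radius.
; While active, a timer-repeated sphere overlap damages a capped number of pawns, optionally sparing the player.
; Each hit spawns two Niagara beams from above and below the tower point, with one zap sound per pulse.
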(event `self.ReceiveBeginPlay`
  (`TimelineComponent.SetPlayRate` (`self.TimelineSpark`) (/ 1.0 (`self.AnimDuration_SparkSphere`)))
  (`SceneComponent.SetHiddenInGame` (`self.NS_SparksActive`) true false))

(event `self.ToggleTrap`
  (set `self.bIsActive` true)
  (`GameplayStatics.PlaySoundAtLocation` "/Game/Audio/SFX/0_Traps/Tesla/SFX_TeslaActive_Cue.SFX_TeslaActive_Cue" (0.0 0.0 0.0) (struct) 1.0 1.0 0.0 null null null null)
  (`|ExecutionSequence`
    (:`then_0`
      (if false
        (`KismetSystemLibrary.DrawDebugSphere` (`SceneComponent.K2_GetComponentLocation` (`self.TeslaTower`)) (`self.Radius`) 12 (struct :`R` 1.0 :`G` 1.0 :`B` 1.0 :`A` 1.0) 2.0)))
    (:`then_1`
      (`self.ToggleSpark` true)
      (`self.DealDamageInArea`)
      (`KismetSystemLibrary.Delay` (`self.ActiveDuration`))
      (`self.ToggleSpark` false)
      (set `self.bIsActive` false))))

(event `ToggleSpark`
  (params (bActive :type Boolean))
  (bind _returnvalue (/ (`self.Radius`) 50.0))
  ;[0.08234 0.14 0.349] Spark animation
  (if bActive
    (`SceneComponent.SetHiddenInGame` (`self.NS_SparksActive`) false false)
    (bind (_direction _alpha) (`Timeline|TimelineSpark` :!via `PlayFromStart` :!label _label)
      (:`Update`
        (`SceneComponent.SetRelativeScale3D` (`self.SparksActive`) (`KismetMathLibrary.VLerp` (0.0 0.0 0.0) (`KismetMathLibrary.MakeVector` _returnvalue _returnvalue _returnvalue) _alpha)))
      (:`Finished`
        (if (not bActive)
          (`SceneComponent.SetHiddenInGame` (`self.NS_SparksActive`) true false))))
    (else
      (goto _label :!via `ReverseFromEnd`))))

(event `DealDamageInArea`
  (bind _enemiesdamagedcounter (`self.EnemiesDamagedCounter`))
  (bind (_returnvalue_x _returnvalue_y _returnvalue_z) (`KismetMathLibrary.BreakVector` (`SceneComponent.K2_GetComponentLocation` (`self.TeslaTower`))))
  (bind (_returnvalue_x_2 _returnvalue_y_2 _returnvalue_z_2) (`KismetMathLibrary.BreakVector` (`SceneComponent.K2_GetComponentLocation` (`self.TeslaTower`))))
  ;[0.1962 0.00826 0] Damage
  (set `self.bCanPlayAudio` true)
  (if (`self.bIsActive`)
    (set `self.EnemiesDamagedCounter` 0)
    (bind _outactors (`KismetSystemLibrary.SphereOverlapActors` (`SceneComponent.K2_GetComponentLocation` (`self.TeslaTower`)) (`self.Radius`) (`|MakeArray` "ObjectTypeQuery3" "ObjectTypeQuery8" :!type "EObjectTypeQuery Enum") "/Script/Engine.Pawn"))
    (for _array_element _outactors
      (`/Engine/EditorBlueprintResources/StandardMacros.IncrementInt` _enemiesdamagedcounter
        (:`  `
          (if (> _enemiesdamagedcounter (`self.MaxPawnsDamaged`))
            (break)
            (elif (== _array_element (`GameplayStatics.GetPlayerPawn` 0))
              (if (`self.bShouldDamagePlayer`)
                (message `IntegrityHolder.Damage` _array_element (`self.Damage`) self :!label _label_2)
                (bind _returnvalue (`NiagaraFunctionLibrary.SpawnSystemAtLocation` "/Game/VFX/Level_VFX/Traps/NS_Zap.NS_Zap"))
                (`FXSystemComponent.SetVectorParameter` _returnvalue "BeamStart" (`KismetMathLibrary.MakeVector` _returnvalue_x_2 _returnvalue_y_2 (+ _returnvalue_z_2 300.0)))
                (`FXSystemComponent.SetVectorParameter` _returnvalue "BeamEnd" (`self.K2_GetActorLocation` _array_element))
                (bind _returnvalue_2 (`NiagaraFunctionLibrary.SpawnSystemAtLocation` "/Game/VFX/Level_VFX/Traps/NS_Zap_02.NS_Zap_02"))
                (`FXSystemComponent.SetVectorParameter` _returnvalue_2 "BeamStart" (`KismetMathLibrary.MakeVector` _returnvalue_x _returnvalue_y (+ _returnvalue_z -300.0)))
                (`FXSystemComponent.SetVectorParameter` _returnvalue_2 "BeamEnd" (`self.K2_GetActorLocation` _array_element))
                (if (`self.bCanPlayAudio`)
                  (set `self.bCanPlayAudio` false)
                  (`GameplayStatics.SpawnSoundAtLocation` (`self.Sound`) (`SceneComponent.K2_GetComponentLocation` (`self.TeslaTower`)) (struct) 1.0 1.0 0.0 null null)))
              (else
                (goto _label_2)))))))
    ;;[0.1962 0.00826 0] New loop
    (`KismetSystemLibrary.K2_SetTimerDelegate` (`|CreateDelegate` :!event `DealDamageInArea`) (`self.DamageTime`))))

(fn `UserConstructionScript`)
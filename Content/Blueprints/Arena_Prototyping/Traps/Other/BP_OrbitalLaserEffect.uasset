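; BP_OrbitalLaserEffect is the visual effect actor for an orbital laser strike, with no damage logic of its own.
; On BeginPlay it activates four laser effects and starts a timeline that narrows the danger decal in Y and Z, then destroys it.
; After a fixed delay from spawn, independent of that timeline, it fires the hit effect and a legacy camera shake.
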(event `self.ReceiveBeginPlay`
  (`ActorComponent.Activate` (`self.NS_Laser1`) false)
  (`ActorComponent.Activate` (`self.NS_Laser2`) false)
  (`ActorComponent.Activate` (`self.NS_Laser3`) false)
  (`ActorComponent.Activate` (`self.NS_Laser4`) false)
  (`self.HideDanger`)
  (`KismetSystemLibrary.Delay` 4.5)
  (`ActorComponent.Activate` (`self.NS_HitEffect`) false)
  (`LegacyCameraShake.StartLegacyCameraShake` null "/Game/Blueprints/RnD/AlphaBlueprints/CameraShake/BP_CameraShakeLegacy_Shoot.BP_CameraShakeLegacy_Shoot_C"))

(event `HideDanger`
  (bind _decal (`self.Decal`))
  (bind (_relative_scale_3d_x _relative_scale_3d_y _relative_scale_3d_z) (`KismetMathLibrary.BreakVector` (`self.Relative Scale 3D`)))
  (set `self.Relative Scale 3D` (`SceneComponent.RelativeScale3D` _decal))
  (bind (_direction _newtrack_0) (`Timeline|Timeline` :!via `PlayFromStart`)
    (:`Update`
      (bind (_returnvalue_x _returnvalue_y _returnvalue_z) (`KismetMathLibrary.BreakVector` (`KismetMathLibrary.VLerp` (`KismetMathLibrary.MakeVector` _relative_scale_3d_x _relative_scale_3d_y _relative_scale_3d_z) (`KismetMathLibrary.MakeVector` _relative_scale_3d_x 0.3 0.3) _newtrack_0)))
      (`SceneComponent.SetRelativeScale3D` _decal (`KismetMathLibrary.MakeVector` _returnvalue_x _returnvalue_y _returnvalue_z)))
    (:`Finished`
      (`ActorComponent.K2_DestroyComponent` (`self.Decal`)))))

(fn `UserConstructionScript`)
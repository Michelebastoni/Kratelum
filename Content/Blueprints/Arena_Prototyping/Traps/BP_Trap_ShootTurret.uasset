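; Arena trap turret that, when toggled, rises, fires projectiles while spinning, then lowers again.
; Two timelines, with play rates set from duration variables, interpolate the turret's height offset and yaw from its starting transform.
; Finishing the rise starts the rotation and a self-rescheduling timer that spawns BP_TurretProjectile at the barrel with muzzle flash and sound.
; Finishing the rotation clears IsActive to stop firing and reverses the move timeline.
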(event `self.ReceiveBeginPlay`
  (`TimelineComponent.SetPlayRate` (`self.TimelineTurret`) (/ 1.0 (`self.TurrentMoveDuration`)))
  (`TimelineComponent.SetPlayRate` (`self.TimelineRotation`) (/ 1.0 (`self.TimeToCompleteRotation`)))
  (set `self.StartingLocation` (`SceneComponent.K2_GetComponentLocation` (`self.Gatling_Turret_Gatling_Turret`)))
  (set `self.StartingRotation` (`SceneComponent.K2_GetComponentRotation` (`self.Gatling_Turret_Gatling_Turret`))))

(event `self.ToggleTrap`
  (set `self.bIsActive` true)
  (`self.MoveTurret` true))

(event `MoveTurret`
  (params (bUp :type Boolean))
  (bind (_startinglocation_x _startinglocation_y _startinglocation_z) (`KismetMathLibrary.BreakVector` (`self.StartingLocation`)))
  (if bUp
    (bind (_direction _alpha) (`Timeline|TimelineTurret` :!via `PlayFromStart` :!label _label)
      (:`Update`
        (`SceneComponent.K2_SetWorldLocation` (`self.Gatling_Turret_Gatling_Turret`) (`KismetMathLibrary.MakeVector` _startinglocation_x _startinglocation_y (+ _startinglocation_z (`KismetMathLibrary.Lerp` 0.0 (`self.HeightOffset`) _alpha))) false false))
      (:`Finished`
        (switch `ETimelineDirection` _direction
          (:`Forward`
            (`self.ShootSequence`)
            (`self.Rotate360Degrees`)))))
    (else
      (goto _label :!via `ReverseFromEnd`))))

(event `ShootSequence`
  (if (`self.bIsActive`)
    (`ActorComponent.Activate` (`self.MuzzleFlash`) true)
    (`|SpawnActorFromClass` "/Game/Blueprints/Arena_Prototyping/Traps/Other/BP_TurretProjectile.BP_TurretProjectile_C" (`SceneComponent.K2_GetComponentToWorld` (`self.TurretBarrel`)) "AlwaysSpawn" "MultiplyWithRoot" null (`self.Damage`) (`self.ProjectileSpeed`) null)
    (`GameplayStatics.PlaySoundAtLocation` (`self.Sound`) (0.0 0.0 0.0) (struct) 1.0 1.0 0.0 null null null null)
    (`KismetSystemLibrary.K2_SetTimerDelegate` (delegate `ShootSequence`) (`self.ShootEvery`))))

(event `Rotate360Degrees`
  (bind (_startingrotation_roll _startingrotation_pitch _startingrotation_yaw) (`KismetMathLibrary.BreakRotator` (`self.StartingRotation`)))
  (bind (_direction _alpha) (`Timeline|TimelineRotation` :!via `PlayFromStart`)
    (:`Update`
      (`SceneComponent.K2_SetWorldRotation` (`self.Gatling_Turret_Gatling_Turret`) (`KismetMathLibrary.MakeRotator` _startingrotation_roll _startingrotation_pitch (`KismetMathLibrary.Lerp` _startingrotation_yaw (+ _startingrotation_yaw (`self.RotationValue`)) _alpha)) false false))
    (:`Finished`
      (set `self.bIsActive` false)
      (`self.MoveTurret` false))))

(fn `UserConstructionScript`)
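; Toggleable spinning-blade trap that makes one round trip between two location markers per trigger, damaging actors it touches.
; ToggleTrap turns on sparks, sound, emissive glow and Tick-driven spin, runs the ping-pong macro, then shuts down.
; A timeline scaled to MovementTime sweeps the blades along local Y, reversing the spin Direction for the return.
; While active, character and enemy hit boxes send DamageMessage after a SkipPlayer check.
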(event `self.ReceiveBeginPlay`
  (`SceneComponent.K2_SetWorldLocation` (`self.Blades`) (`SceneComponent.K2_GetComponentLocation` (`self.LocationA`)) false false)
  (`TimelineComponent.SetPlayRate` (`self.Timeline_MoveTo`) (`KismetMathLibrary.SafeDivide` 1.0 (`self.MovementTime`)))
  (`self.InitBladeMaterials`))

(event `self.ReceiveTick`
  (params (DeltaSeconds :type "Float (single-precision)"))
  ;[1 1 1] Why even compute direction if trap is inactive?
  (if (`self.bIsActive`)
    (bind _output_get (set `self.BladeCurrentSpinningSpeed` (`KismetMathLibrary.FInterpTo` (`self.BladeCurrentSpinningSpeed`) (* (`self.BladeMaxRotationSpeed`) (`self.Direction`)) DeltaSeconds 4.0)))
    (`SceneComponent.K2_AddRelativeRotation` (`self.Blades`) (`KismetMathLibrary.MakeRotator` (* _output_get (`GameplayStatics.GetWorldDeltaSeconds`))) false false)))

(event `self.ToggleTrap`
  ;[0.5203 1 0.4487] Activate Blades
  (`ActorComponent.Activate` (`self.Sparks`) true)
  (`ActorComponent.Activate` (`self.Sparks1`) true)
  (bind _returnvalue (`GameplayStatics.SpawnSoundAtLocation` (`self.Sound`) (`SceneComponent.K2_GetComponentLocation` (`self.Blades`)) (struct) 1.0 1.0 0.0 null null))
  (`self.SetBladesEmissive` (`self.EmissiveStrength`))
  (set `self.bIsActive` true)
  (`self.SetActorTickEnabled` true)
  ;[1 0.8317 0.4394] Move Blades
  (set `self.Direction` 1.0)
  (`KismetSystemLibrary.Delay` 0.5)
  (`self.MoveBladesTo` "NewEnumerator1")
  (`KismetSystemLibrary.Delay` (`self.MovementTime`))
  (set `self.Direction` -1.0)
  (`self.MoveBladesTo` "NewEnumerator0")
  (`KismetSystemLibrary.Delay` (+ (`self.MovementTime`) 0.1))
  ;[1 0.5208 0.5208] Deactivate Blades
  (set `self.bIsActive` false)
  (`self.SetBladesEmissive` 0.0)
  (`ActorComponent.Deactivate` (`self.Sparks`))
  (`ActorComponent.Deactivate` (`self.Sparks1`))
  (`/Engine/EditorBlueprintResources/StandardMacros.IsValid` _returnvalue
    (:`Is Valid`
      (`AudioComponent.Stop` _returnvalue)
      (`self.SetActorTickEnabled` false))))

(event `MoveBladesTo`
  (params (A_or_B :type "/Game/Blueprints/Arena_Prototyping/Traps/Other/ELocations Enum" :default "NewEnumerator0"))
  (bind _blades (`self.Blades`))
  (bind (_relativelocation_x _relativelocation_y _relativelocation_z) (`KismetMathLibrary.BreakVector` (`SceneComponent.RelativeLocation` _blades)))
  (bind (_relativelocation_x_2 _relativelocation_y_2) (`KismetMathLibrary.BreakVector` (`SceneComponent.RelativeLocation` (select `/Game/Blueprints/Arena_Prototyping/Traps/Other/ELocations` A_or_B :`NewEnumerator0` (`self.LocationA`) :`NewEnumerator1` (`self.LocationB`)))))
  (bind (_relativelocation_x_3 _relativelocation_y_3) (`KismetMathLibrary.BreakVector` (`SceneComponent.RelativeLocation` (select `/Game/Blueprints/Arena_Prototyping/Traps/Other/ELocations` A_or_B :`NewEnumerator0` (`self.LocationB`) :`NewEnumerator1` (`self.LocationA`)))))
  (bind (_direction _alpha) (`Timeline|Timeline_MoveTo` :!via `PlayFromStart`)
    (:`Update`
      (`SceneComponent.K2_SetRelativeLocation` _blades (`KismetMathLibrary.MakeVector` _relativelocation_x (`KismetMathLibrary.Lerp` _relativelocation_y_3 _relativelocation_y_2 _alpha) _relativelocation_z) true true))))

(event `self.CharacterHitBox.OnComponentBeginOverlap`
  (params (OverlappedComponent :type "PrimitiveComponent Object Reference") (OtherActor :type "Actor Object Reference") (OtherComp :type "PrimitiveComponent Object Reference") (OtherBodyIndex :type Integer) (bFromSweep :type Boolean) (SweepResult :type "HitResult Structure (by ref)"))
  (if (`self.bIsActive`)
    (`/Game/Blueprints/Arena_Prototyping/MacroLibrary.SkipPlayer?` OtherActor (`self.bShouldDamagePlayer`))
    (message `IntegrityHolder.Damage` OtherActor (`self.Damage`) self)))

(event `self.EnemyHitBox.OnComponentBeginOverlap`
  (params (OverlappedComponent :type "PrimitiveComponent Object Reference") (OtherActor :type "Actor Object Reference") (OtherComp :type "PrimitiveComponent Object Reference") (OtherBodyIndex :type Integer) (bFromSweep :type Boolean) (SweepResult :type "HitResult Structure (by ref)"))
  (if (`self.bIsActive`)
    (`/Game/Blueprints/Arena_Prototyping/MacroLibrary.SkipPlayer?` OtherActor (`self.bShouldDamagePlayer`))
    (message `IntegrityHolder.Damage` OtherActor (`self.Damage`) self)))

(fn `InitBladeMaterials`
  (bind _returnvalue (`PrimitiveComponent.CreateDynamicMaterialInstance` (`self.SM_ConeAround`) 0 "/Game/Materials/Models/BladeSpike/M_GlowSpike_Inst.M_GlowSpike_Inst" "None"))
  (bind _returnvalue_2 (`MaterialInstanceDynamic.K2_GetScalarParameterValue` _returnvalue (`self.EmissiveParamName`)))
  (set `self.EmissiveStrength` _returnvalue_2)
  (`KismetArrayLibrary.Array_Add` (`self.EmissiveMaterialInstances`) _returnvalue)
  (bind _returnvalue_3 (`PrimitiveComponent.CreateDynamicMaterialInstance` (`self.SM_ConeAround1`) 0 "/Game/Materials/Models/BladeSpike/M_GlowSpike_Inst.M_GlowSpike_Inst" "None"))
  (`KismetArrayLibrary.Array_Add` (`self.EmissiveMaterialInstances`) _returnvalue_3)
  (bind _returnvalue_4 (`PrimitiveComponent.CreateDynamicMaterialInstance` (`self.SM_ConeAround2`) 0 "/Game/Materials/Models/BladeSpike/M_GlowSpike_Inst.M_GlowSpike_Inst" "None"))
  (`KismetArrayLibrary.Array_Add` (`self.EmissiveMaterialInstances`) _returnvalue_4)
  (bind _returnvalue_5 (`PrimitiveComponent.CreateDynamicMaterialInstance` (`self.SM_ConeAround3`) 0 "/Game/Materials/Models/BladeSpike/M_GlowSpike_Inst.M_GlowSpike_Inst" "None"))
  (`KismetArrayLibrary.Array_Add` (`self.EmissiveMaterialInstances`) _returnvalue_5)
  (bind _returnvalue_6 (`PrimitiveComponent.CreateDynamicMaterialInstance` (`self.SM_ConeAround4`) 0 "/Game/Materials/Models/BladeSpike/M_GlowSpike_Inst.M_GlowSpike_Inst" "None"))
  (`KismetArrayLibrary.Array_Add` (`self.EmissiveMaterialInstances`) _returnvalue_6)
  (`self.SetBladesEmissive` 0.0))

(fn `SetBladesEmissive`
  (params (NewEmissiveStrength :type "Float (double-precision)"))
  (for _array_element (`self.EmissiveMaterialInstances`)
    (`MaterialInstanceDynamic.SetScalarParameterValue` _array_element (`self.EmissiveParamName`) NewEmissiveStrength))
  (return))

(fn `UserConstructionScript`)
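; Orbital laser trap that, when toggled, spawns a laser effect on SteveJr, chases that character, then explodes.
; Parallel timers schedule the warning cosmetics, the end of tracking, the explosion and effect cleanup.
; Tick interpolates the laser toward its target until tracking stops.
; The explosion damages characters in a sphere around the laser and plays a stronger camera shake if the player is hit.
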(event `self.ToggleTrap`
  (if (not (`self.bIsActive`))
    (`GameplayStatics.PlaySound2D` (`self.Sound_MovingLasers`) 1.0 1.0 0.0 null null)
    ;[0.4222 1 0.6728] Initialize laser effect
    (set `self.bIsActive` true)
    (set `self.CanMoveLaser` true)
    (`self.SpawnLaserEffect`)
    ;[1 0.02604 0.4234] Explosion timer start
    (bind _returnvalue (`KismetSystemLibrary.K2_SetTimerDelegate` (delegate `OnExplosionTimerEnded_Event`) (`self.ExplosionTime`)))
    (set `self.ExplosionTimer` _returnvalue)
    ;[0.09896 0 0.08902] DestroyLaserEffect
    (`KismetSystemLibrary.K2_SetTimerDelegate` (delegate `OnDestroyLaserEnded_Event`) (`self.LaserFXTime`))
    ;[1 0.1198 0.1198] Warning effects timer start
    (bind _returnvalue_2 (`KismetSystemLibrary.K2_SetTimerDelegate` (delegate `OnAnticipationTimerEnded_Event`) (`self.AnticipationTime`)))
    (set `self.AnticipationTimer` _returnvalue_2)
    ;[0.935 0.2865 1] MoveLaser timer start
    (bind _returnvalue_3 (`KismetSystemLibrary.K2_SetTimerDelegate` (delegate `OnMoveLaserTimerEnded_Event`) (`self.MoveLaserTime`)))
    (set `self.MoveLaserTimer` _returnvalue_3)))

(event `OnExplosionTimerEnded_Event`
  ;[1 0.02604 0.4234] Explosion timer start
  (`self.MakeLaserExplosion`))

(event `OnAnticipationTimerEnded_Event`
  ;[1 0.1198 0.1198] Warning effects timer start
  (`self.PerformAnticipationCosmetics`))

(event `OnMoveLaserTimerEnded_Event`
  ;[0.935 0.2865 1] MoveLaser timer start
  (set `self.CanMoveLaser` false))

(event `OnDestroyLaserEnded_Event`
  ;[0.09896 0 0.08902] DestroyLaserEffect
  (`self.K2_DestroyActor` (`self.OrbitalLaser`)))

(event `self.ReceiveTick`
  (params (DeltaSeconds :type "Float (single-precision)"))
  (bind _orbitallaser (`self.OrbitalLaser`))
  (if (and (`self.bIsActive`) (`self.CanMoveLaser`))
    ;[1 0.4938 0.0916] Move laser
    (`self.K2_SetActorLocation` _orbitallaser (`KismetMathLibrary.VInterpTo` (`self.K2_GetActorLocation` _orbitallaser) (`self.K2_GetActorLocation` (`self.LaserTarget`)) DeltaSeconds (`self.LaserSpeed`)) false false)))

(fn `MakeLaserExplosion`
  (bind _returnvalue (`GameplayStatics.GetPlayerController` 0))
  (set `self.bIsActive` false)
  ;[1 0.3365 0.156] Apply Area Damage
  (bind _outactors (`KismetSystemLibrary.SphereOverlapActors` (`self.K2_GetActorLocation` (`self.OrbitalLaser`)) (`self.ExplosionRadius`) (`self.ObjectsToHit`) "/Script/TBO02.GenericCharacter"))
  (for _array_element _outactors
    (message `IntegrityHolder.Damage` _array_element (`self.Damage`) self)
    (if (not (`self.HasHitCharacter`))
      (set `self.HasHitCharacter` (`.bSuccess` (cast `PlayerCharacter` _array_element :!pure true)))))
  ;[0.9865 1 0.142] If player was hit big camera boom else small camera boom
  (if (`self.HasHitCharacter`)
    (`/Game/Blueprints/Cosmetics/CameraShakeClasses/BP_CameraShaker.StrongCameraShake` _returnvalue)
    (else
      (`/Game/Blueprints/Cosmetics/CameraShakeClasses/BP_CameraShaker.WeakCameraShake` _returnvalue 0.2)))
  (set `self.HasHitCharacter` false)
  (`GameplayStatics.PlaySound2D` "/Game/Audio/SFX/0_Traps/Explosions/SFX_Explosion_Barrel_Cue.SFX_Explosion_Barrel_Cue" 1.0 1.0 0.0 null null))

(fn `PerformAnticipationCosmetics`
  (`ActorComponent.Activate` (`/Game/Blueprints/Character_Test/SteveJr.NS_LaserWarning` (`/Game/Blueprints/RnD/BPFunctionsLibrary.GetSteveJr`)) false)
  (`GameplayStatics.PlaySound2D` (`self.Sound`) 1.0 1.0 0.0 null null)
  (`SceneComponent.SetVisibility` (`/Game/Blueprints/Arena_Prototyping/Traps/Other/BP_OrbitalLaserEffect.NS_Laser1` (`self.OrbitalLaser`)) false false)
  (`SceneComponent.SetVisibility` (`/Game/Blueprints/Arena_Prototyping/Traps/Other/BP_OrbitalLaserEffect.NS_Laser2` (`self.OrbitalLaser`)) false false)
  (`SceneComponent.SetVisibility` (`/Game/Blueprints/Arena_Prototyping/Traps/Other/BP_OrbitalLaserEffect.NS_Laser3` (`self.OrbitalLaser`)) false false)
  (`SceneComponent.SetVisibility` (`/Game/Blueprints/Arena_Prototyping/Traps/Other/BP_OrbitalLaserEffect.NS_Laser4` (`self.OrbitalLaser`)) false false))

(fn `SpawnLaserEffect`
  (bind _output_get (set `self.LaserTarget` (`/Game/Blueprints/RnD/BPFunctionsLibrary.GetSteveJr`)))
  (bind _returnvalue (`|SpawnActorFromClass` "/Game/Blueprints/Arena_Prototyping/Traps/Other/BP_OrbitalLaserEffect.BP_OrbitalLaserEffect_C" (`self.GetTransform` _output_get) "Undefined" "MultiplyWithRoot" null null))
  (set `self.OrbitalLaser` _returnvalue))

(fn `UserConstructionScript`)
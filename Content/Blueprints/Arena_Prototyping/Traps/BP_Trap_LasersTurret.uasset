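; BP_Trap_LasersTurret is an arena trap that spins a cube with two damaging laser beams when triggered.
; ToggleTrap only switches it on, showing the laser Niagara effects, playing sound and starting a timeline that sweeps 180 degrees in TimeTo180 seconds.
; While active, Tick runs LaserTrace per emitter with frame-scaled damage, optionally skipping the player.
; The timeline replays for NumberOfRotations, then hides effects, stops sound and resets the trap.
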(event `self.ReceiveBeginPlay`
  (`TimelineComponent.SetPlayRate` (`self.Timeline_Rotate`) (/ 1.0 (`self.TimeTo180`)))
  (set `self.StartRotation` (`SceneComponent.K2_GetComponentRotation` (`self.Cube`))))

(event `self.ToggleTrap`
  (set `self.bIsActive` true)
  (`KismetSystemLibrary.PrintString` "Ehi giampier+" true true (struct :`G` 0.66 :`B` 1.0 :`A` 1.0) 5.0 "asds")
  (bind _returnvalue (`GameplayStatics.SpawnSoundAtLocation` (`self.Sound`) (0.0 0.0 0.0) (struct) 1.0 1.0 0.0 null null))
  (`self.Rotate`)
  (`SceneComponent.SetVisibility` (`self.NS_Laser1`) true false)
  (`SceneComponent.SetVisibility` (`self.NS_Laser2`) true false)
  (`SceneComponent.SetVisibility` (`self.NS_LaserImpact1`) true false)
  (`SceneComponent.SetVisibility` (`self.NS_LaserImpact2`) true false))

(event `self.ReceiveTick`
  (params (DeltaSeconds :type "Float (single-precision)"))
  (if (`self.bIsActive`)
    (`FunctionLibrary.LaserTrace` (`self.LaserEmitter1`) (`self.NS_Laser1`) (`self.NS_LaserImpact1`) (`self.LaserLength1`) (`self.LaserExtendSpeed`) (`self.LaserMaxLength`) (* (`self.DamagePerSecond`) (`GameplayStatics.GetWorldDeltaSeconds`)) (not (`self.bShouldDamagePlayer`)))
    (`FunctionLibrary.LaserTrace` (`self.LaserEmitter2`) (`self.NS_Laser2`) (`self.NS_LaserImpact2`) (`self.LaserLength2`) (`self.LaserExtendSpeed`) (`self.LaserMaxLength`) (* (`self.DamagePerSecond`) (`GameplayStatics.GetWorldDeltaSeconds`)) (not (`self.bShouldDamagePlayer`)))))

(event `Rotate`
  (bind (_startrotation_roll _startrotation_pitch _startrotation_yaw) (`KismetMathLibrary.BreakRotator` (`self.StartRotation`)))
  (bind (_direction _alpha) (`Timeline|Timeline_Rotate` :!via `PlayFromStart` :!label _label)
    (:`Update`
      (`SceneComponent.K2_SetWorldRotation` (`self.Cube`) (`KismetMathLibrary.MakeRotator` _startrotation_roll _startrotation_pitch (+ _startrotation_yaw (`KismetMathLibrary.Lerp` 0.0 180.0 _alpha))) false false))
    (:`Finished`
      (bind _result (`/Engine/EditorBlueprintResources/StandardMacros.IncrementInt` (`self.RotationsDone`))
        (:`  `
          (if (< _result (`self.NumberOfRotations`))
            (goto _label :!via `PlayFromStart`)
            (else
              ;[0 0 0] Turn off
              (`SceneComponent.SetVisibility` (`self.NS_Laser1`) false false)
              (`SceneComponent.SetVisibility` (`self.NS_Laser2`) false false)
              (`SceneComponent.SetVisibility` (`self.NS_LaserImpact1`) false false)
              (`SceneComponent.SetVisibility` (`self.NS_LaserImpact2`) false false)
              (set `self.RotationsDone` 0)
              (`/Engine/EditorBlueprintResources/StandardMacros.IsValid` (stale `self.ToggleTrap` _returnvalue)
                (:`Is Valid`
                  (`AudioComponent.Stop` (stale `self.ToggleTrap` _returnvalue)))
                (:`Is Not Valid`
                  _))
              (set `self.LaserLength1` 0.0)
              (set `self.LaserLength2` 0.0)
              (set `self.bIsActive` false))))))))

(fn `UserConstructionScript`)
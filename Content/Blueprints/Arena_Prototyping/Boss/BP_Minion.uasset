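; BP_Minion is a minion Blueprint for the boss arena prototype, with damage intake, a life bar and toggleable spark effects.
; The Damage event passes value and harmer to HandleDamage, which is defined outside this file.
; UpdateLifeBar sets the W_Lifebar percent from current over starting HP through a widget component.
; SetSparksActivation switches its four Niagara spark effects on or off together.
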(event `self.Damage`
  (params (damageValue :type "Float (single-precision)") (harmer :type "Actor Object Reference"))
  (`self.HandleDamage` damageValue harmer))

(event `self.UpdateLifeBar`
  (bind _w_lifebar (`self.W_Lifebar`))
  (`/Engine/EditorBlueprintResources/StandardMacros.IsValid` _w_lifebar
    (:`Is Valid`
      (bind _asw_lifebar (cast `/Game/Blueprints/Arena_Prototyping/Boss/W_Lifebar` (`WidgetComponent.GetWidget` _w_lifebar)))
      (`ProgressBar.SetPercent` (`/Game/Blueprints/Arena_Prototyping/Boss/W_Lifebar.LifeBar` _asw_lifebar) (/ (`self.CurrentHP`) (`self.StartingHP`))))))

(fn `SetSparksActivation`
  (params (Activate :type Boolean))
  (if Activate
    (`ActorComponent.Activate` (`self.NS_Sparks`) false)
    (`ActorComponent.Activate` (`self.NS_Sparks1`) false)
    (`ActorComponent.Activate` (`self.NS_Sparks2`) false)
    (`ActorComponent.Activate` (`self.NS_Sparks3`) false)
    (else
      (`ActorComponent.Deactivate` (`self.NS_Sparks1`))
      (`ActorComponent.Deactivate` (`self.NS_Sparks`))
      (`ActorComponent.Deactivate` (`self.NS_Sparks2`))
      (`ActorComponent.Deactivate` (`self.NS_Sparks3`)))))

(fn `UserConstructionScript`)
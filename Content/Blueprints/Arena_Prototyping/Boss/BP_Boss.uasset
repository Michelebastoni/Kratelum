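; Prototype arena boss with a life bar and bullet-hell attacks: rotating lasers, minion lasers, projectile bursts from itself or its minions, and spiral waves.
; Each attack is a parameterized event that signals behavior completion, using timelines, delays or looping timers for pacing.
; On Tick, active lasers (two or four) extend gradually, using a line trace for beam and impact visuals and a sphere trace for frame-scaled damage to SteveJr.
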(event `self.ReceiveBeginPlay`
  (set `self.StartRotation` (`SceneComponent.K2_GetComponentRotation` (`self.Lasers`))))

(event `self.Damage`
  (params (damageValue :type "Float (single-precision)") (harmer :type "Actor Object Reference"))
  (`self.HandleDamage` damageValue harmer))

(event `self.ReceiveTick`
  (params (DeltaSeconds :type "Float (single-precision)"))
  (`ProgressBar.SetPercent` (`/Game/Blueprints/Arena_Prototyping/Boss/W_Lifebar.LifeBar` (cast `/Game/Blueprints/Arena_Prototyping/Boss/W_Lifebar` (`WidgetComponent.GetWidget` (`self.W_Lifebar`)) :!pure true)) (/ (`self.CurrentHP`) (`self.StartingHP`)))
  (if (`self.bIsLaserActive`)
    (`self.LaserTrace` (`self.LaserEmitter1`) (`self.NS_Laser1`) (`self.NS_LaserImpact1`) (`self.LaserLength1`))
    (`self.LaserTrace` (`self.LaserEmitter2`) (`self.NS_Laser2`) (`self.NS_LaserImpact2`) (`self.LaserLength2`))
    (`|ExecutionSequence`
      (:`then_0`
        (if (== (`self.CurrNumOfLasers`) 4)
          (`self.LaserTrace` (`self.LaserEmitter3`) (`self.NS_Laser3`) (`self.NS_LaserImpact3`) (`self.LaserLength3`))
          (`self.LaserTrace` (`self.LaserEmitter4`) (`self.NS_Laser4`) (`self.NS_LaserImpact4`) (`self.LaserLength4`)))))))

(event `Rotate`
  (params (NumOfRotations :type Integer))
  (bind (_startrotation_roll _startrotation_pitch _startrotation_yaw) (`KismetMathLibrary.BreakRotator` (`self.StartRotation`)))
  (bind (_direction _alpha) (`Timeline|Timeline_Rotation` :!via `PlayFromStart` :!label _label)
    (:`Update`
      (`SceneComponent.K2_SetWorldRotation` (`self.Lasers`) (`KismetMathLibrary.MakeRotator` _startrotation_roll _startrotation_pitch (+ _startrotation_yaw (`KismetMathLibrary.Lerp` 0.0 360.0 _alpha))) false false))
    (:`Finished`
      (bind _result (`/Engine/EditorBlueprintResources/StandardMacros.IncrementInt` (`self.RotationsDone`))
        (:`  `
          (if (< _result NumOfRotations)
            (goto _label :!via `PlayFromStart`)
            (else
              ;[0 0 0] Turn off
              (`SceneComponent.SetVisibility` (`self.NS_Laser1`) false false)
              (`SceneComponent.SetVisibility` (`self.NS_Laser2`) false false)
              (`SceneComponent.SetVisibility` (`self.NS_Laser3`) false false)
              (`SceneComponent.SetVisibility` (`self.NS_Laser4`) false false)
              (`SceneComponent.SetVisibility` (`self.NS_LaserImpact1`) false false)
              (`SceneComponent.SetVisibility` (`self.NS_LaserImpact2`) false false)
              (`SceneComponent.SetVisibility` (`self.NS_LaserImpact3`) false false)
              (`SceneComponent.SetVisibility` (`self.NS_LaserImpact4`) false false)
              (set `self.RotationsDone` 0)
              (set `self.LaserLength1` 0.0)
              (set `self.LaserLength2` 0.0)
              (set `self.LaserLength3` 0.0)
              (set `self.LaserLength4` 0.0)
              (set `self.bIsLaserActive` false)
              (`self.OnFinishBehavior`))))))))

(event `MinionLasersAtk`
  (params (LaserSpeed :type "Float (single-precision)" :default 500.0) (HowMany :type Integer) (DelayBetween :type "Float (double-precision)" :default 1.0) (AnticipationDuration :type "Float (single-precision)"))
  ;[1 1 1] Laser minions
  (set `self.MinionLaserAnticipationDuration` AnticipationDuration)
  (if (> HowMany 0)
    (set `self.i` 0)
    (`self.MinionsLaserAttack` LaserSpeed :!label _label_2)
    (bind _result (`/Engine/EditorBlueprintResources/StandardMacros.IncrementInt` (`self.i`))
      (:`  `
        (if (< _result HowMany)
          (`KismetSystemLibrary.Delay` DelayBetween)
          (goto _label_2)
          (else
            (`KismetSystemLibrary.Delay` (+ (`KismetMathLibrary.SafeDivide` 2000.0 LaserSpeed) (`self.MinionLaserAnticipationDuration`)))
            (`self.OnFinishBehavior`)))))
    (else
      (`KismetSystemLibrary.PrintString` "Error LaserMinions: HowMany <= 0 ")
      (`self.OnFinishBehavior`))))

(event `BurstFromBoss`
  (params (Duration :type "Float (single-precision)" :default 10.0) (SpawnDelay :type "Float (single-precision)" :default 0.1) (AngleVariance :type "Float (single-precision)" :default 18.0) (SpeedVarianceMult :type "Float (single-precision)" :default 0.5) (BaseSpeed :type "Float (double-precision)" :default 600.0))
  ;[1 1 1] Spawn single difficult burst
  (`self.SpawnBurstTowardPlayer` Duration SpawnDelay AngleVariance SpeedVarianceMult (make `ProjectileParameters` (`self.K2_GetActorLocation`) (struct) 1.2 BaseSpeed 8.0))
  (`KismetSystemLibrary.Delay` Duration)
  (`self.OnFinishBehavior`))

(event `SpiralWave`
  (params (Duration :type "Float (single-precision)" :default 10.0) (Frequency :type "Float (double-precision)" :default 0.5) (ChangeDirectionProbability :type "Float (double-precision)") (RotationAngle :type "Float (double-precision)" :default 10.0) (ProjectileSpeed :type "Float (single-precision)" :default 600.0) (SpawnPointCount :type Integer :default 3))
  ;[1 1 1] Spiral wave
  (set `self.CurrSpiralDirection` 1.0)
  (bind _returnvalue (`KismetSystemLibrary.K2_SetTimerDelegate` (delegate `SpiralWave_ev`) Frequency true))
  (`KismetSystemLibrary.Delay` Duration)
  (`KismetSystemLibrary.K2_ClearAndInvalidateTimerHandle` _returnvalue)
  (`self.OnFinishBehavior`))

(event `SpiralWave_ev`
  (bind (_returnvalue_x _returnvalue_y _returnvalue_z) (`KismetMathLibrary.BreakVector` (`self.K2_GetActorLocation`)))
  ;[1 1 1] Spiral wave
  (`self.SpawnProjectiles` (stale `SpiralWave` SpawnPointCount) 200.0 (`self.CurrentOffset`) (make `ProjectileParameters` (`KismetMathLibrary.MakeVector` _returnvalue_x _returnvalue_y (+ _returnvalue_z (`self.ProjectilesHeight`))) (struct) 1.0 (stale `SpiralWave` ProjectileSpeed) 10.0))
  (if (< (`KismetMathLibrary.RandomFloat`) (stale `SpiralWave` ChangeDirectionProbability))
    (set `self.CurrSpiralDirection` (* (`self.CurrSpiralDirection`) -1.0)))
  (set `self.CurrentOffset` (+ (`self.CurrentOffset`) (* (/ (`KismetMathLibrary.GetPI`) (stale `SpiralWave` RotationAngle)) (`self.CurrSpiralDirection`)))))

(event `BurstFromMinions`
  (params (Duration :type "Float (single-precision)" :default 5.0) (SpawnDelay :type "Float (double-precision)" :default 0.15) (AngleVariance :type "Float (double-precision)" :default 15.0) (SpeedVarianceMult :type "Float (double-precision)" :default 0.4))
  ;[1 1 1] Spawn medium burst from all the minions
  (`self.BuststMinions` Duration SpawnDelay AngleVariance SpeedVarianceMult)
  (`KismetSystemLibrary.Delay` Duration)
  (`self.OnFinishBehavior`))

(event `Laser`
  (params (TimeTo360 :type "Float (double-precision)") (NumOfLasers :type Integer) (NumOfRotations :type Integer))
  ;[1 1 1] Laser
  (set `self.CurrNumOfLasers` NumOfLasers)
  (`TimelineComponent.SetPlayRate` (`self.Timeline_Rotation`) (`KismetMathLibrary.SafeDivide` 1.0 TimeTo360))
  (set `self.bIsLaserActive` true)
  (switch `int` (`self.CurrNumOfLasers`)
    (:`Default`
      (`KismetSystemLibrary.PrintString` "Error Laser: wrong lasers active." :!label _label_3)
      (`self.OnFinishBehavior`))
    (:`2`
      (`SceneComponent.SetVisibility` (`self.NS_Laser1`) true false)
      (`SceneComponent.SetVisibility` (`self.NS_Laser2`) true false)
      (`SceneComponent.SetVisibility` (`self.NS_LaserImpact1`) true false)
      (`SceneComponent.SetVisibility` (`self.NS_LaserImpact2`) true false)
      (`self.Rotate` NumOfRotations :!label _label_4))
    (:`3`
      (goto _label_3))
    (:`4`
      (`SceneComponent.SetVisibility` (`self.NS_Laser1`) true false)
      (`SceneComponent.SetVisibility` (`self.NS_Laser2`) true false)
      (`SceneComponent.SetVisibility` (`self.NS_Laser4`) true false)
      (`SceneComponent.SetVisibility` (`self.NS_Laser3`) true false)
      (`SceneComponent.SetVisibility` (`self.NS_LaserImpact1`) true false)
      (`SceneComponent.SetVisibility` (`self.NS_LaserImpact2`) true false)
      (`SceneComponent.SetVisibility` (`self.NS_LaserImpact3`) true false)
      (`SceneComponent.SetVisibility` (`self.NS_LaserImpact4`) true false)
      (goto _label_4))))

(fn `BuststMinions`
  (params (Duration :type "Float (double-precision)") (SpawnDelay :type "Float (double-precision)") (AngleVariance :type "Float (double-precision)") (SpeedVarianceMult :type "Float (double-precision)"))
  (for _array_element (`self.Minions`)
    (`/Engine/EditorBlueprintResources/StandardMacros.IsValid` _array_element
      (:`Is Valid`
        (`self.SpawnBurstTowardPlayer` (`local.Duration`) (`local.SpawnDelay`) (`local.AngleVariance`) (`local.SpeedVarianceMult`) (make `ProjectileParameters` (`self.K2_GetActorLocation` _array_element) (struct) 1.0 1.0 8.0))))))

(fn `LaserTrace`
  (params (LaserOrigin :type "StaticMeshComponent Object Reference") (NS_Laser :type "NiagaraComponent Object Reference") (NS_LaserImpact :type "NiagaraComponent Object Reference") (LaserLength :type "Float (double-precision) (by ref)"))
  (locals (bHasHit :type Boolean :default false) (ImpactLocation :type "Vector Structure" :default (0.0 0.0 0.0)))
  (bind _returnvalue (`SceneComponent.K2_GetComponentLocation` (`local.LaserOrigin`)))
  (bind _returnvalue_2 (`SceneComponent.K2_GetComponentLocation` (`local.LaserOrigin`)))
  (bind _returnvalue_3 (+ _returnvalue_2 (* (`SceneComponent.GetForwardVector` (`local.LaserOrigin`)) (`local.LaserLength`))))
  (`|ExecutionSequence`
    (:`then_0`
      ;[0 0 0] Laser visual
      (bind (_outhit _returnvalue_4) (`KismetSystemLibrary.LineTraceSingle` _returnvalue_2 _returnvalue_3 "TraceTypeQuery1"))
      (set `local.bHasHit` _returnvalue_4)
      (bind (_bblockinghit _binitialoverlap _time _distance _location _impactpoint) (`GameplayStatics.BreakHitResult` _outhit))
      (set `local.ImpactLocation` _impactpoint)
      (`NiagaraComponent.SetVariableVec3` (`local.NS_Laser`) "BeamEnd" (`KismetMathLibrary.SelectVector` _impactpoint _returnvalue_3 (`local.bHasHit`)))
      (`SceneComponent.SetVisibility` (`local.NS_LaserImpact`) (`local.bHasHit`) false)
      (`SceneComponent.K2_SetWorldLocation` (`local.NS_LaserImpact`) (`local.ImpactLocation`) false false))
    (:`then_1`
      ;[0 0 0] Damage
      (bind _outhits (`KismetSystemLibrary.SphereTraceMultiByProfile` _returnvalue (+ _returnvalue (* (`SceneComponent.GetForwardVector` (`local.LaserOrigin`)) (`local.LaserLength`))) (`self.LaserRadius`) "Pawn" false (`|MakeArray` self :!type "Actor Object Reference")))
      (for _array_element _outhits
        (bind (_bblockinghit_2 _binitialoverlap_2 _time_2 _distance_2 _location_2 _impactpoint_2 _normal _impactnormal _physmat _hitactor) (`GameplayStatics.BreakHitResult` _array_element))
        (cast `/Game/Blueprints/Character_Test/SteveJr` _hitactor)
        (message `IntegrityHolder.Damage` _hitactor (* (`self.DamagePerSecond`) (`GameplayStatics.GetWorldDeltaSeconds`)) self)))
    (:`then_2`
      ;[0 0 0] New laser length
      (if (< (`local.LaserLength`) (`self.LaserMaxLength`))
        (`|VariableSetRef` (`local.LaserLength`) (`KismetMathLibrary.FClamp` (+ (`local.LaserLength`) (* (`GameplayStatics.GetWorldDeltaSeconds`) (`self.LaserExtendSpeed`))) 0.0 (`self.LaserMaxLength`)))))))

(fn `UpdateLifeBar`
  (bind _w_lifebar (`self.W_Lifebar`))
  (`/Engine/EditorBlueprintResources/StandardMacros.IsValid` _w_lifebar
    (:`Is Valid`
      (bind _asw_lifebar (cast `/Game/Blueprints/Arena_Prototyping/Boss/W_Lifebar` (`WidgetComponent.GetWidget` _w_lifebar)))
      (`ProgressBar.SetPercent` (`/Game/Blueprints/Arena_Prototyping/Boss/W_Lifebar.LifeBar` _asw_lifebar) (/ (`self.CurrentHP`) (`self.StartingHP`))))))

(fn `UserConstructionScript`)
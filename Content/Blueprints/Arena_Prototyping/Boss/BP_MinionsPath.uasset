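; Boss arena prototype path that shifts a group of minions one point along a looping four-point spline per MoveToNextPoint call.
; A movement timeline, rate set by MovementDuration, slides minions at evenly staggered, wrapped spline times, then a rotation timeline turns them to their point's rotation.
; Sparks show during movement, while hitboxes and metallic friction sound last until rotation ends.
; The self-timed loop is disconnected, so nothing here triggers the move.
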(event `self.ReceiveBeginPlay`
  (bind _spline (`self.Spline`))
  (`TimelineComponent.SetPlayRate` (`self.Timeline_Movement`) (`KismetMathLibrary.SafeDivide` 1.0 (`self.MovementDuration`)))
  (set `self.TimeDistanceBetweenPoints` (/ (`SplineComponent.Duration` _spline) (`SplineComponent.GetNumberOfSplinePoints` _spline))))

(event `MoveToNextPoint`
  (bind _returnvalue (`GameplayStatics.SpawnSound2D` "/Game/Audio/SFX/Boss/SFX_MetallicFriction_Cue.SFX_MetallicFriction_Cue" 1.0 1.0 0.0 null))
  (set `self.SFX_Metallic` _returnvalue)
  (bind _result (`/Engine/EditorBlueprintResources/StandardMacros.IncrementInt` (`self.CurrentPoint`))
    (:`  `
      (if (> _result 4)
        (set `self.CurrentPoint` 1))
      (for _array_element (`self.Minions`)
        (`/Engine/EditorBlueprintResources/StandardMacros.IsValid` _array_element
          (:`Is Valid`
            (`/Game/Blueprints/Arena_Prototyping/Boss/BP_Minion.SetSparksActivation` _array_element true)
            (`PrimitiveComponent.SetCollisionEnabled` (`Minion.HitBox` _array_element) "QueryAndPhysics"))))
      ;[0 0 0] Movement
      (bind (_direction _alpha) (`Timeline|Timeline_Movement` :!via `PlayFromStart`)
        (:`Update`
          (for (_array_element_2 _array_index) (`self.Minions`)
            (`/Engine/EditorBlueprintResources/StandardMacros.IsValid` _array_element_2
              (:`Is Valid`
                (bind _returnvalue_2 (+ (* _array_index (`self.TimeDistanceBetweenPoints`)) (`KismetMathLibrary.MapRangeClamped` _alpha 0.0 1.0 (* (`self.TimeDistanceBetweenPoints`) (- (`self.CurrentPoint`) 1)) (* (`self.TimeDistanceBetweenPoints`) (`self.CurrentPoint`)))))
                (`self.K2_SetActorLocation` _array_element_2 (`SplineComponent.GetLocationAtTime` (`self.Spline`) (`KismetMathLibrary.SelectFloat` (`KismetMathLibrary.Fraction` _returnvalue_2) _returnvalue_2 (> _returnvalue_2 1.0)) "World" false) false false)))))
        (:`Finished`
          (for _array_element_3 (`self.Minions`)
            (`/Engine/EditorBlueprintResources/StandardMacros.IsValid` _array_element_3
              (:`Is Valid`
                (`/Game/Blueprints/Arena_Prototyping/Boss/BP_Minion.SetSparksActivation` _array_element_3 false))))
          ;[0 0 0] Rotation
          (bind (_direction_2 _alpha_2) (`Timeline|Timeline_Rotation` :!via `PlayFromStart`)
            (:`Update`
              (for (_array_element_4 _array_index_2) (`self.Minions`)
                (`/Engine/EditorBlueprintResources/StandardMacros.IsValid` _array_element_4
                  (:`Is Valid`
                    (bind _returnvalue_3 (+ _array_index_2 (`self.CurrentPoint`)))
                    (`self.K2_SetActorRotation` _array_element_4 (`KismetMathLibrary.RLerp` (`self.K2_GetActorRotation` _array_element_4) (`SplineComponent.GetRotationAtSplinePoint` (`self.Spline`) (`KismetMathLibrary.SelectInt` (- _returnvalue_3 4) _returnvalue_3 (> _returnvalue_3 3)) "World") _alpha_2 true) false)))))
            (:`Finished`
              (`AudioComponent.Stop` (`self.SFX_Metallic`))
              (for _array_element_5 (`self.Minions`)
                (`/Engine/EditorBlueprintResources/StandardMacros.IsValid` _array_element_5
                  (:`Is Valid`
                    (`PrimitiveComponent.SetCollisionEnabled` (`Minion.HitBox` _array_element_5) "NoCollision")))))))))))

(fn `UserConstructionScript`)
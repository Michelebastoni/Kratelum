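; BP_HealingBase is a boss arena prototype actor that heals BP_Boss when a Minion enters its sphere.
; After a short delay, the overlap tints its dynamic material orange and starts HealBoss, then turns it black once HealDuration elapses.
; HealBoss re-arms a timer to heal in ticks derived from amount, duration and rate, resetting its total on reaching HealAmount without applying that last tick.
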(event `self.ReceiveBeginPlay`
  (bind _returnvalue (`GameplayStatics.GetActorOfClass` "/Game/Blueprints/Arena_Prototyping/Boss/BP_Boss.BP_Boss_C"))
  (set `self.Boss` _returnvalue)
  (set `self.HealingPerTick` (* (/ (`self.HealAmount`) (`self.HealDuration`)) (`self.HealTickRate`))))

(event `self.SphereCollision.OnComponentBeginOverlap`
  (params (OverlappedComponent :type "PrimitiveComponent Object Reference") (OtherActor :type "Actor Object Reference") (OtherComp :type "PrimitiveComponent Object Reference") (OtherBodyIndex :type Integer) (bFromSweep :type Boolean) (SweepResult :type "HitResult Structure (by ref)"))
  (cast `Minion` OtherActor)
  (`KismetSystemLibrary.Delay` 0.5)
  (`MaterialInstanceDynamic.SetVectorParameterValue` (`self.M_Base`) "Color" (struct :`R` 1.0 :`G` 0.494898 :`A` 1.0))
  (set `self.bIsHealing` true)
  (`self.HealBoss`)
  (`KismetSystemLibrary.Delay` (`self.HealDuration`))
  (set `self.bIsHealing` false)
  (`MaterialInstanceDynamic.SetVectorParameterValue` (`self.M_Base`) "Color" (struct :`A` 1.0)))

(event `HealBoss`
  (bind _output_get (set `self.HealingDone` (+ (`self.HealingDone`) (`self.HealingPerTick`))))
  (if (< _output_get (`self.HealAmount`))
    (`Boss.Heal` (`self.Boss`) (`self.HealingPerTick`))
    (`KismetSystemLibrary.K2_SetTimerDelegate` (delegate `HealBoss`) (`self.HealTickRate`))
    (else
      (set `self.HealingDone` 0.0))))

(fn `UserConstructionScript`
  (bind _returnvalue (`PrimitiveComponent.CreateDynamicMaterialInstance` (`self.SM_HealingBase`) 0 "/Game/Materials/SolidColors/M_SolidColor_Gray.M_SolidColor_Gray" "None"))
  (set `self.M_Base` _returnvalue))
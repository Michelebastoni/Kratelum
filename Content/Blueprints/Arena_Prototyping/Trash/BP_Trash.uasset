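; BP_Trash is an arena prototype trash prop that removes itself when its ClearTrash event is called.
; ClearTrash activates a Niagara effect, waits, then starts a looping timer that flip-flops the trash mesh's hidden state so it blinks.
; After a short blink period it clears the timer, activates the puff effect and destroys the actor immediately.
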(event `self.ReceiveBeginPlay`)

(event `ClearTrash`
  (bind _blinkingtimer (`self.BlinkingTimer`))
  (`ActorComponent.Activate` (`self.Niagara`) false)
  (`KismetSystemLibrary.Delay` 5.0)
  (bind _returnvalue (`KismetSystemLibrary.K2_SetTimerDelegate` (delegate `MeshVisibility`) 0.3 true))
  (set `self.BlinkingTimer` _returnvalue)
  (`KismetSystemLibrary.Delay` 3.0)
  (if (`KismetSystemLibrary.K2_IsValidTimerHandle` _blinkingtimer)
    (`KismetSystemLibrary.K2_ClearAndInvalidateTimerHandle` _blinkingtimer)
    (`ActorComponent.Activate` (`self.NS_Puff`) false)
    (`self.K2_DestroyActor`)))

(event `MeshVisibility`
  (bind _sm_trashcombined1 (`self.SM_TrashCombined1`))
  (`/Engine/EditorBlueprintResources/StandardMacros.FlipFlop`
    (:`A`
      (`SceneComponent.SetHiddenInGame` _sm_trashcombined1 true false))
    (:`B`
      (`SceneComponent.SetHiddenInGame` _sm_trashcombined1 false false))))

(fn `UserConstructionScript`)
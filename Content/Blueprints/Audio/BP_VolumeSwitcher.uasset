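; BP_VolumeSwitcher is an interactable hit target that applies one music or SFX volume preset from its audio config, likely in the hub.
; Switchers in a group listen to each other's change events, so the invoker sets the volume through LoopStationSubsystem and spins, while same-class siblings reverse.
; Outline color and icon emissive show the active preset, initialized from saved settings.
; A flip-flop timeline rotates the switcher in or out, gating interaction.
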(event `self.ReceiveBeginPlay`
  (`self.Setup`)
  (for _array_element (`self.SwitchersGroup`)
    (add `self.OnAudioSettingValueChanged` _array_element (delegate `OnAudioSettingValueChanged_Event`))
    (`self.Event Toggle`)))

(event `OnAudioSettingValueChanged_Event` :!signature `self.OnAudioSettingValueChanged`
  (params (Invoker :type "/Game/Blueprints/Audio/BP_VolumeSwitcher Object Reference"))
  (bind _isself (`self.HandleOnAudioSettingValueChanged` Invoker))
  (if _isself
    (bind (_direction _high_button) (`Timeline|RotateTimeline` :!label _label)
      (:`Update`
        (`SceneComponent.K2_SetRelativeRotation` (`self.Pern`) (`KismetMathLibrary.MakeRotator` 0.0 0.0 (* _high_button -360.0)) false false))
      (:`Finished`
        (`/Game/Blueprints/HUB_Elements/Settigs/Setting_Buttons/Setting_Sign/BP_SoundIcon.ToggleEmissive` (`self.TogglableSoundIcon`) _isself)
        (`self.ToggleOutlineColor` _isself)))
    (else
      (goto _label :!via `Reverse`))))

(event `self.Interact`
  (params (Interactor :type "Interactor Interface (by ref)") (InteractionMethod :type "EInteractionMethod Enum" :default "KeyPress"))
  (bind _returnvalue (`Interactable.CanInteract` Interactor InteractionMethod))
  (if _returnvalue
    (`self.OnAudioSettingValueChanged` self)
    (`GameplayStatics.PlaySoundAtLocation` (`self.HitSound`) (0.0 0.0 0.0) (struct) 1.0 1.0 0.0 null null null null)))

(event `Event Toggle`
  (`/Engine/EditorBlueprintResources/StandardMacros.FlipFlop`
    (:`A`
      (bind (_direction _settings_anim) (`Timeline|T_ToggleSettings` :!label _label_2)
        (:`Update`
          (`SceneComponent.K2_SetRelativeRotation` (`self.Pern`) (`KismetMathLibrary.MakeRotator` (* _settings_anim (`self.ToggleRotation`))) false false))
        (:`Finished`
          (if (== (`self.ToggleRotation`) 90.0)
            (set `self.IsToggled` true)
            (set `self.IsAnimating` false)
            (elif (== (`self.ToggleRotation`) 0.0)
              (set `self.IsToggled` false)
              (set `self.IsAnimating` false)
              (else
                (set `self.IsAnimating` true)))))))
    (:`B`
      (goto _label_2 :!via `Reverse`))))

(fn `CanInteract`
  (params (Interactor :type "Interactor Interface (by ref)") (InteractionMethod :type "EInteractionMethod Enum" :default "KeyPress"))
  (returns (ReturnValue :type Boolean))
  (bind _t_togglesettings (`self.T_ToggleSettings`))
  (return (and (not (or (`TimelineComponent.IsPlaying` _t_togglesettings) (`TimelineComponent.IsReversing` _t_togglesettings))) (`self.IsToggled`))))

(fn `HandleOnAudioSettingValueChanged`
  (params (Invoker :type "/Game/Blueprints/Audio/BP_VolumeSwitcher Object Reference"))
  (returns (IsSelf :type Boolean))
  (locals (IsSelfValue :type Boolean))
  (bind _audioconfigdata (`self.AudioConfigData`))
  (if (== Invoker self)
    (`LoopStationSubsystem.SetVolume` (subsystem `LoopStationSubsystem`) (`/Game/Blueprints/Audio/Data/BP_AudioSwitchPreset.SoundMix` _audioconfigdata) (`/Game/Blueprints/Audio/Data/BP_AudioSwitchPreset.SoundClass` _audioconfigdata) (`/Game/Blueprints/Audio/Data/BP_AudioSwitchPreset.IsMusic` _audioconfigdata) (`/Game/Blueprints/Audio/Data/BP_AudioSwitchPreset.VolumePreset` _audioconfigdata))
    (return true)
    (elif (== (`/Game/Blueprints/Audio/BP_VolumeSwitcher.SoundClassTarget` Invoker) (`self.SoundClassTarget`))
      (return false))))

(fn `Setup`
  (bind _audioconfigdata (`self.AudioConfigData`))
  (bind _sm_setting_target (`self.SM_Setting_target`))
  (bind _volumepreset (`/Game/Blueprints/Audio/Data/BP_AudioSwitchPreset.VolumePreset` _audioconfigdata))
  (bind _returnvalue (`PrimitiveComponent.CreateDynamicMaterialInstance` _sm_setting_target 0 (`MeshComponent.GetOverlayMaterial` _sm_setting_target) "None"))
  (bind _output_get (set `self.TargetOutline` _returnvalue))
  (`MeshComponent.SetOverlayMaterial` _sm_setting_target _output_get)
  (`PrimitiveComponent.SetMaterial` (`self.SM_Setting_target`) 0 "/Game/Materials/HUB_Material/M_Setting/M_Target_HUB.M_Target_HUB")
  (set `self.SoundClassTarget` (`/Game/Blueprints/Audio/Data/BP_AudioSwitchPreset.SoundClass` _audioconfigdata))
  (if (`/Game/Blueprints/Audio/Data/BP_AudioSwitchPreset.IsMusic` _audioconfigdata)
    (bind _returnvalue_2 (`LoopStationSubsystem.GetMusicSettings`))
    (if (`|EnumEquality` _volumepreset _returnvalue_2)
      (`/Game/Blueprints/HUB_Elements/Settigs/Setting_Buttons/Setting_Sign/BP_SoundIcon.ToggleEmissive` (`self.TogglableSoundIcon`) true :!label _label)
      (`self.ToggleOutlineColor` true)
      (else
        (`self.ToggleOutlineColor` false :!label _label_2)))
    (else
      (bind _returnvalue_3 (`LoopStationSubsystem.GetSfxSettings`))
      (if (`|EnumEquality` _returnvalue_3 _volumepreset)
        (goto _label)
        (else
          (goto _label_2))))))

(fn `ToggleOutlineColor`
  (params (IsSelf :type Boolean))
  (if IsSelf
    (`MaterialInstanceDynamic.SetVectorParameterValue` (`self.TargetOutline`) "OutlineColor" (`self.ActiveOutlineCol`))
    (else
      (`MaterialInstanceDynamic.SetVectorParameterValue` (`self.TargetOutline`) "OutlineColor" (`self.InactiveOutlineCol`)))))

(fn `UserConstructionScript`)
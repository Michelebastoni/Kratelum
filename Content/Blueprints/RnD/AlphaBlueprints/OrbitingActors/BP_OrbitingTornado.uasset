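; BP_OrbitingTornado is an actor, named as a tornado, that circles a target actor in the horizontal plane.
; Each Tick calls Orbit, which advances CurrentAngle by speed times delta time, wrapped at 360 degrees.
; It then uses cosine and sine scaled by Radius to set its location around the target's current position, at the target's height, without sweeping.
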(event `self.ReceiveBeginPlay`)

(event `self.ReceiveTick`
  (params (DeltaSeconds :type "Float (single-precision)"))
  (`self.Orbit` (`self.Target Center`) (`self.Orbit Speed`) DeltaSeconds (`self.Current Angle`) (`self.Radius`)))

(fn `Orbit`
  (params (TargetCenter :type "Actor Object Reference") (OrbitSpeed :type "Float (double-precision)") (DeltaTime :type "Float (double-precision)") (CurrentAngle :type "Float (double-precision) (by ref)") (Radius :type "Float (double-precision)"))
  (bind _output_get (set `self.Current Angle` (mod (+ (* OrbitSpeed DeltaTime) CurrentAngle) 360.0)))
  (bind _returnvalue (`KismetMathLibrary.DegreesToRadians` _output_get))
  (`self.K2_SetActorLocation` (+ (`self.K2_GetActorLocation` TargetCenter) (`KismetMathLibrary.MakeVector` (* (`KismetMathLibrary.Cos` _returnvalue) Radius) (* (`KismetMathLibrary.Sin` _returnvalue) Radius)))))

(fn `UserConstructionScript`)
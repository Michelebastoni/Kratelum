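; BP_AudioLoopTrigger is an R&D trigger that adds an audio loop when something overlaps its collision component.
; On BeginPlay, a text component shows the uppercased name of the loop in LoopData, or a red "UNINITIALIZED!" warning if either is invalid.
; On overlap, it validates LoopData and its LoopToPlay, then passes LoopData to AddLoop with no fade-in, without filtering the overlapping actor.
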(event `self.ReceiveBeginPlay`
  (bind _loopdata (`self.LoopData`))
  (bind _loopnametext (`self.LoopNameText`))
  (bind _looptoplay (`AudioSwitchTrackData.LoopToPlay` _loopdata))
  (`/Engine/EditorBlueprintResources/StandardMacros.IsValid` _loopdata
    (:`Is Valid`
      (`/Engine/EditorBlueprintResources/StandardMacros.IsValid` _looptoplay
        (:`Is Valid`
          (`TextRenderComponent.K2_SetText` _loopnametext (`KismetTextLibrary.Conv_StringToText` (`KismetStringLibrary.ToUpper` (`KismetSystemLibrary.GetObjectName` _looptoplay)))))
        (:`Is Not Valid`
          (`TextRenderComponent.K2_SetText` _loopnametext (`KismetTextLibrary.Conv_StringToText` "UNINITIALIZED!") :!label _label)
          (`TextRenderComponent.SetTextRenderColor` _loopnametext (`KismetMathLibrary.Conv_LinearColorToColor` (`KismetMathLibrary.LinearColor_Red`))))))
    (:`Is Not Valid`
      (goto _label))))

(event `self.CollisionComponent.OnComponentBeginOverlap`
  (params (OverlappedComponent :type "PrimitiveComponent Object Reference") (OtherActor :type "Actor Object Reference") (OtherComp :type "PrimitiveComponent Object Reference") (OtherBodyIndex :type Integer) (bFromSweep :type Boolean) (SweepResult :type "HitResult Structure (by ref)"))
  (bind _loopdata (`self.LoopData`))
  (`/Engine/EditorBlueprintResources/StandardMacros.IsValid` _loopdata
    (:`Is Valid`
      (`/Engine/EditorBlueprintResources/StandardMacros.IsValid` (`AudioSwitchTrackData.LoopToPlay` _loopdata)
        (:`Is Valid`
          (`LoopStationSubsystem.AddLoop` _loopdata))))))

(fn `UserConstructionScript`)
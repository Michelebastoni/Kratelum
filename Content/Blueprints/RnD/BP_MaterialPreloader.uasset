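; BP_MaterialPreloader is an R&D actor that sweeps through a list of target points, apparently to preload materials along the route.
; Each tick it teleports toward the current point at a fixed high speed, moving only in XY and keeping its own height.
; It advances the index when a point is within one step, and after the last it fires a finished-travel delegate, prints a message and stops.
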(event `self.ReceiveTick`
  (params (DeltaSeconds :type "Float (single-precision)"))
  (bind (_returnvalue_x _returnvalue_y _returnvalue_z) (`KismetMathLibrary.BreakVector` (`self.K2_GetActorLocation`)))
  (bind (_returnvalue_x_2 _returnvalue_y_2 _returnvalue_z_2) (`KismetMathLibrary.BreakVector` (`self.K2_GetActorLocation`)))
  (bind (_returnvalue_x_3 _returnvalue_y_3) (`KismetMathLibrary.BreakVector` (`self.K2_GetActorLocation` (`|GetArrayItem` (`self.TargetPoints`) (`self.CurrIndex`)))))
  (if (not (`self.HasDone`))
    (bind _output_get (set `self.TargetPos` (`KismetMathLibrary.MakeVector` _returnvalue_x_3 _returnvalue_y_3 _returnvalue_z)))
    (bind _output_get_2 (set `self.StartPos` (`self.K2_GetActorLocation`)))
    (bind _output_get_3 (set `self.DistVec` (- _output_get _output_get_2)))
    (set `self.DistLength` (`KismetMathLibrary.VSize` _output_get_3))
    (bind _output_get_4 (set `self.MoveStep` (* DeltaSeconds 5000.0)))
    (if (<= (`self.DistLength`) _output_get_4)
      (bind _result (`/Engine/EditorBlueprintResources/StandardMacros.IncrementInt` (`self.CurrIndex`))
        (:`  `
          (if (>= _result (`KismetArrayLibrary.Array_Length` (`self.TargetPoints`)))
            (`self.OnFinishedTravelDelegate`)
            (`KismetSystemLibrary.PrintString` "FINISHED TRAVELLING!")
            (set `self.HasDone` true))))
      (else
        (bind _output_get_5 (set `self.Direction` (`KismetMathLibrary.Normal` (`self.DistVec`))))
        (bind _output_get_6 (set `self.NewLoc` (+ (`self.StartPos`) (* _output_get_5 (`self.MoveStep`)))))
        (`self.K2_SetActorLocation` (`KismetMathLibrary.MakeVector` (.x _output_get_6) (.y _output_get_6) _returnvalue_z_2) false true)))))

(fn `UserConstructionScript`)
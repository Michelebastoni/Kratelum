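; BP_ArenaEventDispatcher ends an arena level when the Score Handler signals a level win.
; After a delay it plays a victory sound and, unless EnemiesToKill is -1, compares the current score with the target score.
; It then shows either the Win or Survived screen with score, level name and next level, and saves the score data through ScoreSaveSystem.
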(event `self.ReceiveBeginPlay`
  (`parent.ReceiveBeginPlay`)
  (`self.ScoreHandler`
    (:`then`
      (add `self.OnLevelWonDelegate` (delegate `OnLevelWonDelegate_Event`)))
    (:`else`
      (`KismetSystemLibrary.PrintText` (`|FormatText` "Score Handler not set into {name}" (`KismetSystemLibrary.GetDisplayName` self)) true false (struct :`R` 1.0 :`G` 0.241945 :`A` 1.0)))))

(event `OnLevelWonDelegate_Event` :!signature `self.OnLevelWonDelegate`
  (params (LevelIndex :type Integer))
  (`KismetSystemLibrary.Delay` (`self.TimeToWait`))
  (`GameplayStatics.PlaySound2D` "/Game/Audio/SFX/0_Game/GameWin/SFX_GameVictorySound_Cue.SFX_GameVictorySound_Cue" 1.0 1.0 0.0 null null)
  (if (not (== (`self.EnemiesToKill`) -1))
    (`self.HandleEndLevel`)))

(fn `HandleEndLevel`
  (`self.TriggerEndScreen` (>= (`ScoreHandler.GetCurrentScore` (`self.ScoreHandler`)) (`self.Score_To_Reach`))))

(fn `SaveGame`
  (bind _returnvalue (`GameplayStatics.CreateSaveGameObject` "/Script/TBO02.ScoreSaveSystem"))
  (`ScoreSaveSystem.SetScoreData` _returnvalue (`self.ScoreHandler`) (`self.Level_Data_ToSave`)))

(fn `TriggerEndScreen`
  (params (`bWin?` :type Boolean))
  ;[0 0 0] To be optimized if possible
  (if `bWin?`
    (bind _returnvalue (`|CreateWidget` "/Game/Blueprints/Widgets/EndScreen_Widget/WBP_Win_Screen.WBP_Win_Screen_C"))
    (`WinScreen.SetNextLevelToLoad` _returnvalue (`self.Level_To_Load`))
    (`/Game/Blueprints/Widgets/EndScreen_Widget/WBP_Win_Screen.SetUpScoreDisplay` _returnvalue (`self.ScoreHandler`))
    (`/Game/Blueprints/Widgets/EndScreen_Widget/WBP_Win_Screen.SetLevelText` _returnvalue (`self.LevelName`))
    (`UserWidget.AddToViewport` _returnvalue 0)
    (`GameScreen.ToggleGameScreen` _returnvalue true)
    (else
      (bind _returnvalue_2 (`|CreateWidget` "/Game/Blueprints/Widgets/EndScreen_Widget/WBP_Survived_Screen.WBP_Survived_Screen_C"))
      (`WinScreen.SetNextLevelToLoad` _returnvalue_2 (`self.Level_To_Load`))
      (`/Game/Blueprints/Widgets/EndScreen_Widget/WBP_Survived_Screen.SetUpScoreDisplay` _returnvalue_2 (`self.ScoreHandler`))
      (`/Game/Blueprints/Widgets/EndScreen_Widget/WBP_Survived_Screen.SetLevelText` _returnvalue_2 (`self.LevelName`))
      (`UserWidget.AddToViewport` _returnvalue_2 0)
      (`GameScreen.ToggleGameScreen` _returnvalue_2 true)))
  (`self.SaveGame`))

(fn `UserConstructionScript`)
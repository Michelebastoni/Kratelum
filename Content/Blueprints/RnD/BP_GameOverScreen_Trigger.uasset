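; Level-placed trigger actor that shows the game over screen when the player character dies.
; On BeginPlay it creates the WBP_GameOver_Screen widget, adds it to the viewport and binds to player 0's GenericCharacter death event, printing an error if that cast fails.
; On death it plays a game over voice cue, waits briefly, then toggles the screen on.
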(event `self.ReceiveBeginPlay`
  (`|ExecutionSequence`
    (:`then_0`
      ;[0 0 0] Create GameOver Widget and add into viewport
      (bind _returnvalue (`|CreateWidget` "/Game/Blueprints/Widgets/EndScreen_Widget/WBP_GameOver_Screen.WBP_GameOver_Screen_C"))
      (bind _output_get (set `self.GameOverWidget` _returnvalue))
      (`UserWidget.AddToViewport` _output_get 1))
    (:`then_1`
      ;[0 0 0] Find player and bind character dead event
      (bind _asgeneric_character (cast `GenericCharacter` (`GameplayStatics.GetPlayerCharacter` 0))
        (:`then`
          (add `GenericCharacter.OnCharacterDeath` _asgeneric_character (delegate `HandleCharacterDeath`)))
        (:`CastFailed`
          (`KismetSystemLibrary.PrintText` (`|FormatText` "CANT FIND PLAYER CHARACTER \nSource:  {Name}" (`KismetSystemLibrary.GetDisplayName` self)) true false (struct :`R` 1.0 :`A` 1.0) 1000.0 "Error"))))))

(event `HandleCharacterDeath`
  (params (character :type "GenericCharacter Object Reference") (currentWeapon :type "Weapon Object Reference") (harmer :type "Actor Object Reference") (integrity :type "Integrity Object Reference"))
  ;[0 0 0] Find player and bind character dead event
  (`GameplayStatics.PlaySound2D` "/Game/Audio/SFX/0_Game/Game_Over/SFX_GameOverSoundVoice_Cue.SFX_GameOverSoundVoice_Cue" 1.0 1.0 0.0 null null)
  (`KismetSystemLibrary.Delay` 2.5)
  (`GameScreen.ToggleGameScreen` (`self.GameOverWidget`) true))

(fn `UserConstructionScript`)
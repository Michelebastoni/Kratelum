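; Cinematic actor that plays a skippable level sequence, either at level start or when triggered through CreateLevelSequence.
; On start it switches the controller to cinematic context, fades the HUD and, given a ScoreHandler, fades score and hides the player.
; Skipping jumps to the end, and stopping fires a finish notification.
; With BindToLSFinished, spawners pause during playback, then the view blends from this actor to the player before input and spawning resume.
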(event `self.ReceiveBeginPlay`
  (`self.Level Sequence`
    (:`then`
      (if (`self.bPlayAtStart`)
        (`self.CreateLevelSequence`)))
    (:`else`)))

(event `self.ReceiveEndPlay`
  (params (EndPlayReason :type "EEndPlayReason Enum" :default "Destroyed"))
  (bind _as_generic_player_controller (`self.As Generic Player Controller`))
  ;[0 0 0] Get Controller + HUD reference and hide it on start
  (`/Engine/EditorBlueprintResources/StandardMacros.IsValid` _as_generic_player_controller
    (:`Is Valid`
      (if (`self.bPlayAtStart`)
        (remove `GenericPlayerController.OnFinishSetUp` _as_generic_player_controller (delegate `SetUpPlayerSettings`)))
      (remove `GenericPlayerController.OnSkipCinematic` _as_generic_player_controller (delegate `On_SkipEvent`)))))

(event `SetUpPlayerSettings`
  (params (Player_Controller :type "GenericPlayerController Object Reference"))
  (bind _scorehandler (`self.ScoreHandler`))
  (bind _output_get (set `self.HUD_Screen` (`GenericPlayerController.GetHUDScreen` Player_Controller)))
  (`HUDWidget.PlayFadeAnimation` _output_get false 1.0)
  (`GenericPlayerController.SwitchIntoCinematicContext` (`self.As Generic Player Controller`))
  (`/Engine/EditorBlueprintResources/StandardMacros.IsValid` _scorehandler
    (:`Is Valid`
      (`ScoreWidget.PlayScore_Fade` (`ScoreHandler.GetScoreWidget` _scorehandler) false 2.0)
      (`KismetSystemLibrary.DelayUntilNextTick`)
      (set `self.Current_Player` (`GenericPlayerController.GetCurrentCharacter` Player_Controller))
      (`self.TogglePlayerVisiblity` false))))

(event `On_SkipEvent`
  (bind _lsp (`self.LSP`))
  ;[0 0 0] Get Controller + HUD reference and hide it on start
  (if (and (`KismetSystemLibrary.IsValid` _lsp) (`MovieSceneSequencePlayer.IsPlaying` _lsp))
    (`MovieSceneSequencePlayer.GoToEndAndStop` _lsp)
    (`Widget.RemoveFromParent` (`self.SkipWidget`))))

(event `CreateLevelSequence`
  (`|ExecutionSequence`
    (:`then_0`
      ;[0 0 0] Get Controller + HUD reference and hide it on start
      (bind _output_get (set `self.As Generic Player Controller` (cast `GenericPlayerController` (`GameplayStatics.GetPlayerController` 0) :!pure true)))
      (if (`self.bPlayAtStart`)
        (add `GenericPlayerController.OnFinishSetUp` _output_get (delegate `SetUpPlayerSettings`))
        (else
          (`self.SetUpPlayerSettings` _output_get)))
      (add `GenericPlayerController.OnSkipCinematic` _output_get (delegate `On_SkipEvent`)))
    (:`then_1`
      ;[0 0 0] Create and add skip widget + start Level sequence
      (bind _returnvalue (`|CreateWidget` "/Game/Blueprints/Widgets/Cinematic_Widget/WBP_Skip_Cinematic.WBP_Skip_Cinematic_C"))
      (bind _output_get_2 (set `self.SkipWidget` _returnvalue))
      (`UserWidget.AddToViewport` _output_get_2 0)
      (bind (_outactor _returnvalue_2) (`LevelSequencePlayer.CreateLevelSequencePlayer` (`self.Level Sequence`) (`self.Settings`)))
      (bind _output_get_3 (set `self.LSP` _returnvalue_2))
      (`MovieSceneSequencePlayer.Play` _output_get_3)
      (add `MovieSceneSequencePlayer.OnStop` _output_get_3 (delegate `Notify LSP_End`))
      (if (`self.bBindToLSFinished`)
        (add `MovieSceneSequencePlayer.OnStop` (`self.LSP`) (delegate `OnSequenceStop`))
        (for _array_element (`self.PowerUpSpawners`)
          (`/Game/Blueprints/Arena_Prototyping/Loot/BP_LootPowerUpSpawner.StopSpawner` _array_element))
        (for _array_element_2 (`self.WeaponSpawner`)
          (`/Game/Blueprints/Arena_Prototyping/Loot/BP_LootWeaponSpawner.StopSpawner` _array_element_2))))))

(event `Notify LSP_End`
  ;[0 0 0] Create and add skip widget + start Level sequence
  (`self.OnCinematicFinish`))

(event `OnSequenceStop`
  ;[0 0 0] Create and add skip widget + start Level sequence
  (`self.ToggleHUD`)
  (`self.TogglePlayerVisiblity` true)
  (`KismetSystemLibrary.Delay` (`self.Camera_Blend_time`))
  (bind _enemy_spawner (`self.Enemy_Spawner`)
    (:`then`
      (`EnemySpawner.StartSpawner` _enemy_spawner))
    (:`else`
      _))
  (for _array_element (`self.PowerUpSpawners`)
    (set `/Game/Blueprints/Arena_Prototyping/Loot/BP_LootPowerUpSpawner.bCanSpawn` true _array_element))
  (for _array_element_2 (`self.WeaponSpawner`)
    (set `/Game/Blueprints/Arena_Prototyping/Loot/BP_LootWeaponSpawner.bCanSpawn` true _array_element_2)))

(fn `GiveInput`
  (bind _scorehandler (`self.ScoreHandler`))
  (bind _as_generic_player_controller (`self.As Generic Player Controller`))
  (`/Engine/EditorBlueprintResources/StandardMacros.IsValid` _as_generic_player_controller
    (:`Is Valid`
      (`GenericPlayerController.SwitchIntoGameContext` _as_generic_player_controller)
      (`HUDWidget.PlayFadeAnimation` (`self.HUD_Screen`) true 0.0)
      (`Widget.RemoveFromParent` (`self.SkipWidget`))
      (`/Engine/EditorBlueprintResources/StandardMacros.IsValid` _scorehandler
        (:`Is Valid`
          (`ScoreWidget.PlayScore_Fade` (`ScoreHandler.GetScoreWidget` _scorehandler) true 0.0)
          (`self.K2_DestroyActor`))))))

(fn `SetUp`
  (bind _returnvalue (`GameplayStatics.GetActorOfClass` "/Script/TBO02.ScoreHandler"))
  (set `self.ScoreHandler` _returnvalue)
  (bind _returnvalue_2 (`GameplayStatics.GetActorOfClass` "/Game/Blueprints/SpawningSystem/BP_EnemySpawnerInst.BP_EnemySpawnerInst_C"))
  (set `self.Enemy_Spawner` _returnvalue_2)
  (bind _outactors (`GameplayStatics.GetAllActorsOfClass` "/Game/Blueprints/Arena_Prototyping/Loot/BP_LootPowerUpSpawner.BP_LootPowerUpSpawner_C"))
  (set `self.PowerUpSpawners` _outactors)
  (bind _outactors_2 (`GameplayStatics.GetAllActorsOfClass` "/Game/Blueprints/Arena_Prototyping/Loot/BP_LootWeaponSpawner.BP_LootWeaponSpawner_C"))
  (set `self.WeaponSpawner` _outactors_2))

(fn `ToggleHUD`
  (bind _as_generic_player_controller (`self.As Generic Player Controller`))
  (if (`KismetSystemLibrary.IsValid` _as_generic_player_controller)
    (`PlayerController.SetViewTargetWithBlend` _as_generic_player_controller self 0.0 "VTBlend_Linear" 0.0 false)
    (`PlayerController.SetViewTargetWithBlend` _as_generic_player_controller (`GenericPlayerController.GetCurrentCharacter` _as_generic_player_controller) (`self.Camera_Blend_time`) "VTBlend_EaseOut" 1.0 false)
    (`KismetSystemLibrary.K2_SetTimer` null "GiveInput" (`self.Camera_Blend_time`))))

(fn `TogglePlayerVisiblity`
  (params (Show :type Boolean))
  (bind _returnvalue (`GenericCharacter.GetCurrentWeapon` (`self.Current_Player`)))
  (`/Engine/EditorBlueprintResources/StandardMacros.IsValid` (`self.Current_Player`)
    (:`Is Valid`
      (if Show
        (`self.SetActorHiddenInGame` _returnvalue false)
        (`self.SetActorHiddenInGame` (`self.Current_Player`) false)
        (else
          (`self.SetActorHiddenInGame` _returnvalue true)
          (`self.SetActorHiddenInGame` (`self.Current_Player`) true))))))

(fn `UserConstructionScript`)